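; Grabbable laptop actor whose screen hinges open and closed by following a hand position.
; Pickup attaches it to the given component with keyboard physics off; Drop detaches it and restores physics.
; StartTracking opens a Tick gate that derives a signed pivot-to-hand angle, flips it by keyboard orientation, and sets pivot roll within min/max limits.
; An older world-rotation approach remains unwired, and Tick prints a debug orientation vector.
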(event Custom|StopTracking
  (Actor|Tick|SetActorTickEnabled false)
  (Utilities|FlowControl|Gate true) ; enters at Close
)

(event Custom|StartTracking
  (Actor|Tick|SetActorTickEnabled true)
  (Utilities|FlowControl|Gate true) ; enters at Open
)

(event EventBeginPlay
  (Variables|Default|SetScreenRotate (Variables|/Script/Engine.SceneComponent|GetRelativeRotation (Variables|Default|GetPivot)))
  (Variables|Default|SetHandHoldPosition (Transformation|GetWorldLocation (Variables|Default|GetBP_LaptopHandPoint))))

(event EventPickup
  (params (AttachTo :type Scene%20Component%20Object%20Reference))
  (Actor|Tick|SetActorTickEnabled true)
  (Physics|SetSimulatePhysics (Variables|Default|GetKeyBoard) false)
  (Transformation|AttachComponentToComponent (VehicleSound|GetRootComponent) AttachTo "None" "KeepWorld" "KeepWorld" "KeepWorld" false))

(event EventTick
  (params (DeltaSeconds :type Float%20%28single-precision%29))
  (Development|PrintString (Utilities|String|ToString(Vector) (Class|KismetMathLibrary|VectorGetSignVector (Math|Rotator|GetRotationXVector (Transformation|GetWorldRotation (Variables|Default|GetKeyBoard))))))
  (Utilities|FlowControl|Gate true
    (:Exit
      (Variables|Default|SetNewScreenRotate (Variables|/Script/Engine.SceneComponent|GetRelativeRotation (Variables|Default|GetPivot)))
      (Variables|Default|SetCurrentAngle (CallFunction|GetScreenAngle))
      (if (< (Math|Float|Absolute(Float) (Variables|Default|GetCurrentAngle)) 125.0)
        (if (< (.x (Class|KismetMathLibrary|VectorGetSignVector (Math|Rotator|GetRotationXVector (Transformation|GetWorldRotation (Variables|Default|GetKeyBoard))))) 0.0)
          _
          (else
            (Variables|Default|SetCurrentAngle (* (CallFunction|GetScreenAngle) -1.0))))
        (if (<= (Variables|Default|GetCurrentAngle) (Variables|Default|GetMinAngle))
          (Transformation|SetRelativeRotation (Variables|Default|GetPivot) (Math|Rotator|MakeRotator (|MinAngleOnlyX) 0.0 0.0) false false)
          (elif (not (>= (Variables|Default|GetCurrentAngle) (Variables|Default|GetMaxAngle)))
            (Transformation|SetRelativeRotation (Variables|Default|GetPivot) (Math|Rotator|MakeRotator (|GetAngleOnlyx) 0.0 0.0) false false)))))))

(event EventDrop
  (Actor|Tick|SetActorTickEnabled false)
  (Physics|SetSimulatePhysics (Variables|Default|GetKeyBoard) true)
  (Transformation|DetachFromActor "KeepWorld" "KeepWorld" "KeepWorld"))

(fn ConstructionScript)

(fn GetScreenRotation
  (params (OpationalDirection :type Vector) (UseDirection :type Boolean))
  (return (Class|KismetMathLibrary|MakeRotfromYZ (Math|Vector|SelectVector OpationalDirection (CallFunction|GetHandDire) UseDirection) (CallFunction|GetRightVectorSelf))))

(fn GetHandDire
  (return (Math|Vector|Normalize (- (Variables|Default|GetHandPosition) (Transformation|GetWorldLocation (Variables|Default|GetPivot))))))

(fn GetScreenAngle
  (return (* (Class|KismetMathLibrary|DegAcos (Math|Vector|DotProduct (CallFunction|GetHandDire) (CallFunction|GetForwardVectorSelf))) (Math|Float|SelectFloat -1.0 1.0 (< (.x (Math|Vector|CrossProduct (CallFunction|GetHandDire) (CallFunction|GetForwardVectorSelf))) 0.0)))))

(fn GetRightVectorSelf
  (return (Math|Vector|Normalize (- (Transformation|GetWorldLocation (Variables|Default|GetLP)) (Transformation|GetWorldLocation (Variables|Default|GetRP))))))

(fn GetForwardVectorSelf
  (return (Math|Vector|Normalize (- (Transformation|GetWorldLocation (Variables|Default|GetFP)) (Transformation|GetWorldLocation (Variables|Default|GetPivot))))))