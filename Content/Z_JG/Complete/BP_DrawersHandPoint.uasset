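; Grabbable hand point for a drawer, used as a child actor of BP_Drawers to stand in for the handle while held.
; Pickup attaches it to the grabbing component and opens a gated Tick that turns the drawer on and feeds it the sphere's position as HandPosition.
; Drop moves the sphere back to the last sampled handle location, detaches, turns the drawer off and closes the gate.
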(event EventBeginPlay
  (bind _asbp_drawers (Utilities|Casting|CastToBP_Drawers (Actor|GetParentActor)))
  (bind _output_get (Variables|Default|SetHandPointLocation (Transformation|GetWorldLocation (Variables|/Game/Z_JG/Complete/BP_Drawers.BP_Drawers_C|GetHandle _asbp_drawers))))
  (Variables|Default|SetHandPointNewLocation _output_get))

(event EventTick
  (params (DeltaSeconds :type Float%20%28single-precision%29))
  (Utilities|FlowControl|Gate true
    (:Exit
      (bind _asbp_drawers (Utilities|Casting|CastToBP_Drawers (Actor|GetParentActor)))
      (Variables|Default|SetHandPointLocation (Transformation|GetWorldLocation (Variables|/Game/Z_JG/Complete/BP_Drawers.BP_Drawers_C|GetHandle _asbp_drawers)))
      (Variables|Default|SetHandPointNewLocation (Transformation|GetWorldLocation (Variables|Default|GetSphere)))
      (CallFunction|TurnonPoint))))

(event EventPickup
  (params (AttachTo :type Scene%20Component%20Object%20Reference))
  (Actor|Tick|SetActorTickEnabled true)
  (Transformation|AttachComponentToComponent (VehicleSound|GetRootComponent) AttachTo "None" "KeepWorld" "KeepWorld" "KeepWorld" false)
  (Utilities|FlowControl|Gate true) ; enters at Open
)

(event EventDrop
  (Actor|Tick|SetActorTickEnabled false)
  (Transformation|SetWorldLocation (Variables|Default|GetSphere) (Variables|Default|GetHandPointLocation) false false)
  (Transformation|DetachFromActor "KeepWorld" "KeepWorld" "KeepWorld")
  (CallFunction|TurnOffPoint)
  (Utilities|FlowControl|Gate true) ; enters at Close
)

(fn ConstructionScript)

(fn TurnonPoint
  (bind _asbp_drawers (Utilities|Casting|CastToBP_Drawers (Actor|GetParentActor)))
  (Default|Turnon _asbp_drawers)
  (Variables|/Game/Z_JG/Complete/BP_Drawers.BP_Drawers_C|SetHandPosition _asbp_drawers (Transformation|GetWorldLocation (Variables|Default|GetSphere))))

(fn TurnOffPoint
  (bind _asbp_drawers (Utilities|Casting|CastToBP_Drawers (Actor|GetParentActor)))
  (Default|TurnOff _asbp_drawers)
  (Variables|/Game/Z_JG/Complete/BP_Drawers.BP_Drawers_C|SetHandPosition _asbp_drawers (Transformation|GetWorldLocation (Variables|Default|GetSphere))))

(fn TurnonDrawer
  (params (HandPoint :type Vector :default "0, 0, 0"))
  (return))