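; BP_MicrowaveTimerHandPoint is the grabbable handle point for the timer knob on BP_Microwave.
; Pickup attaches it to the grabbing component and opens a gated Tick that records the grip location and handle rotation, calling TimerStart and passing that rotation to the parent microwave.
; Drop snaps the handle to the grip, keeping only the new roll, reattaches it and calls TimerStop with the final rotation.
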(event EventBeginPlay
  (Variables|컴포넌트|SetGrip (Class|Actor|GetParentComponent))
  (Variables|Default|SetDoor_HandPointLocation (Transformation|GetWorldLocation (Variables|컴포넌트|GetGrip)))
  (Variables|Default|SetTimer_HandPointRotate (Transformation|GetWorldRotation (Variables|Default|GetPointHandle))))

(event EventTick
  (params (DeltaSeconds :type Float%20%28single-precision%29))
  (Utilities|FlowControl|Gate true
    (:Exit
      (Variables|Default|SetDoor_HandPointLocation (Transformation|GetWorldLocation (Variables|컴포넌트|GetGrip)))
      (Variables|Default|SetTimer_HandPointNewRotate (Transformation|GetWorldRotation (Variables|Default|GetPointHandle)))
      (CallFunction|TurnonPoint))))

(event EventPickup
  (params (AttachTo :type Scene%20Component%20Object%20Reference))
  (Actor|Tick|SetActorTickEnabled true)
  (Transformation|AttachComponentToComponent (VehicleSound|GetRootComponent) AttachTo "None" "KeepWorld" "KeepWorld" "KeepWorld" false)
  (Utilities|FlowControl|Gate true) ; enters at Open
)

(event EventDrop
  (bind _timer_handpointrotate (Variables|Default|GetTimer_HandPointRotate))
  (bind (_roll _pitch _yaw) (Math|Rotator|BreakRotator _timer_handpointrotate))
  (Actor|Tick|SetActorTickEnabled false)
  (Transformation|SetWorldLocation (Variables|Default|GetPointHandle) (Variables|Default|GetDoor_HandPointLocation) false false)
  (Transformation|SetWorldRotation (Variables|Default|GetPointHandle) (Math|Rotator|MakeRotator (.Roll (Math|Rotator|BreakRotator (Variables|Default|GetTimer_HandPointNewRotate))) _pitch _yaw) false false)
  (Transformation|DetachFromActor "KeepWorld" "KeepWorld" "KeepWorld")
  (Transformation|AttachComponentToComponent (VehicleSound|GetRootComponent) (Variables|컴포넌트|GetGrip) "None" "KeepWorld" "KeepWorld" "KeepWorld" false)
  (CallFunction|TurnOffPoint)
  (Utilities|FlowControl|Gate true) ; enters at Close
)

(fn ConstructionScript)

(fn TurnonPoint
  (bind _asbp_microwave (Utilities|Casting|CastToBP_Microwave (Actor|GetParentActor)))
  (Default|TimerStart _asbp_microwave)
  (Variables|/Game/Z_JG/Complete/BP_Microwave.BP_Microwave_C|SetTimerHandRotate _asbp_microwave (Variables|Default|GetTimer_HandPointNewRotate)))

(fn TurnOffPoint
  (bind _asbp_microwave (Utilities|Casting|CastToBP_Microwave (Actor|GetParentActor)))
  (Default|TimerStop _asbp_microwave)
  (Variables|/Game/Z_JG/Complete/BP_Microwave.BP_Microwave_C|SetTimerHandRotate _asbp_microwave (Variables|Default|GetTimer_HandPointNewRotate)))