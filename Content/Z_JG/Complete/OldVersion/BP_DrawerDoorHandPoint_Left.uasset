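; Grabbable hand point for the left drawer door, a child actor that relays the grabbing hand's position to its parent BP_DrawerDoor_Left.
; Pickup attaches it to the grabber and opens a Tick gate that starts door tracking and feeds the Sphere's location as HandPosition.
; Drop snaps the Sphere to the grip's last recorded location, reattaches the actor to the grip, and stops tracking.
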(event EventBeginPlay
  (Variables|Default|SetGrip (Class|Actor|GetParentComponent))
  (bind _output_get (Variables|Default|SetDoor_HandPointLocation (Transformation|GetWorldLocation (Variables|Default|GetGrip))))
  (Variables|Default|SetDoor_HandPointNewLocation _output_get))

(event EventTick
  (params (DeltaSeconds :type Float%20%28single-precision%29))
  (Utilities|FlowControl|Gate true
    (:Exit
      (Variables|Default|SetDoor_HandPointLocation (Transformation|GetWorldLocation (Variables|Default|GetGrip)))
      (Variables|Default|SetDoor_HandPointNewLocation (Transformation|GetWorldLocation (Variables|Default|GetSphere)))
      (CallFunction|TurnonPoint))))

(event EventPickup
  (params (AttachTo :type Scene%20Component%20Object%20Reference))
  (Actor|Tick|SetActorTickEnabled true)
  (Transformation|AttachComponentToComponent (VehicleSound|GetRootComponent) AttachTo "None" "KeepWorld" "KeepWorld" "KeepWorld" false)
  (Utilities|FlowControl|Gate true) ; enters at Open
)

(event EventDrop
  (Actor|Tick|SetActorTickEnabled false)
  (Transformation|SetWorldLocation (Variables|Default|GetSphere) (Variables|Default|GetDoor_HandPointLocation) false false)
  (Transformation|DetachFromActor "KeepWorld" "KeepWorld" "KeepWorld")
  (Transformation|AttachComponentToComponent (VehicleSound|GetRootComponent) (Variables|Default|GetGrip) "None" "KeepWorld" "KeepWorld" "KeepWorld" false)
  (CallFunction|TurnOffPoint)
  (Utilities|FlowControl|Gate true) ; enters at Close
)

(fn ConstructionScript)

(fn TurnonPoint
  (bind _asbp_drawer_door_left (Utilities|Casting|CastToBP_DrawerDoor_Left (Actor|GetParentActor)))
  (Default|StartTracking _asbp_drawer_door_left)
  (Variables|/Game/Z_JG/Complete/OldVersion/BP_DrawerDoor_Left.BP_DrawerDoor_Left_C|SetHandPosition _asbp_drawer_door_left (Variables|Default|GetDoor_HandPointNewLocation)))

(fn TurnOffPoint
  (bind _asbp_drawer_door_left (Utilities|Casting|CastToBP_DrawerDoor_Left (Actor|GetParentActor)))
  (Default|StopTracking _asbp_drawer_door_left)
  (Variables|/Game/Z_JG/Complete/OldVersion/BP_DrawerDoor_Left.BP_DrawerDoor_Left_C|SetHandPosition _asbp_drawer_door_left (Variables|Default|GetDoor_HandPointNewLocation)))