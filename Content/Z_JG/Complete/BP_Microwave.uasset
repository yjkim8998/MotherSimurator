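; Interactive VR microwave with a hand-driven door, timer dial, start button, spinning plate and interior light.
; Externally called start/stop events gate Tick, which swings the door toward HandPosition between angle limits or applies TimerHandRotate to the dial.
; A motion controller overlapping the button starts a Delay loop that winds the timer down and spins the plate while the door is closed.
; The light follows door and cooking state, and the button resets when time runs out.
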(event OnComponentBeginOverlap(Button)
  (params (OverlappedComponent :type Primitive%20Component%20Object%20Reference) (OtherActor :type Actor%20Object%20Reference) (OtherComp :type Primitive%20Component%20Object%20Reference) (OtherBodyIndex :type Integer) (bFromSweep :type Boolean) (SweepResult :type Hit%20Result%20Structure%20%28by%20ref%29))
  (if (not (Variables|Default|GetStartButton))
    (if (> (- (.roll (Variables|Default|GetTimerNewRotate)) (.roll (Variables|Default|GetTimerRotate))) 2.0)
      (Utilities|Casting|CastToBP_MotionController OtherActor)
      (Transformation|AddRelativeLocation (Variables|Default|GetButton) "-5.000000, 0, 0" false false)
      (Variables|Default|SetStartButton true)
      (if (> (- (.roll (Variables|Default|GetTimerNewRotate)) (.roll (Variables|Default|GetTimerRotate))) 2.0) :!label _label
        (if (not (Variables|Default|GetDoorOpen))
          (if (Variables|Default|GetStartButton)
            (Rendering|SetVisibility (Variables|Default|GetPointLight) true false)
            (Transformation|AddRelativeRotation (Variables|Default|GetBP_MicrowaveTimer) (Math|Rotator|MakeRotator -0.5 0.0 0.0) false false)
            (Variables|Default|SetTimerNewRotate (Variables|/Script/Engine.SceneComponent|GetRelativeRotation (Variables|Default|GetBP_MicrowaveTimer)))
            (Transformation|AddRelativeRotation (Variables|Default|GetPlate) (Math|Rotator|MakeRotator 0.0 0.0 3.0) false false)
            (Transformation|SetRelativeRotation (Variables|Default|GetBP_MicrowaveTimerHandPoint) (Variables|Default|GetTimerNewRotate) false false)
            (Utilities|FlowControl|Delay 0.1)
            (goto _label)))
        (else
          (Rendering|SetVisibility (Variables|Default|GetPointLight) false false)
          (Transformation|SetWorldLocation (Variables|Default|GetButton) (Variables|Default|GetButtonOrginalPosition) false false)
          (Variables|Default|SetStartButton false))))))

(event Custom|StopTracking
  (Variables|Default|SetDoorController false)
  (Actor|Tick|SetActorTickEnabled false)
  (Utilities|FlowControl|Gate true) ; enters at Close
)

(event Custom|StartTracking
  (Variables|Default|SetDoorController true)
  (Actor|Tick|SetActorTickEnabled true)
  (Utilities|FlowControl|Gate true) ; enters at Open
)

(event Custom|TimerStop
  (Variables|Default|SetTimerController false)
  (Actor|Tick|SetActorTickEnabled false)
  (Utilities|FlowControl|Gate true) ; enters at Close
)

(event Custom|TimerStart
  (Variables|Default|SetTimerController true)
  (Actor|Tick|SetActorTickEnabled true)
  (Utilities|FlowControl|Gate true) ; enters at Open
)

(event EventBeginPlay
  (Variables|Default|SetInitDoorDirection (Math|Vector|GetRightVector (Variables|Default|GetDoorPivot)))
  (Variables|Default|SetDoorRotate (Transformation|GetWorldRotation (Variables|Default|GetDoorPivot)))
  (Variables|Default|SetTimerNewRotate (Variables|/Script/Engine.SceneComponent|GetRelativeRotation (Variables|Default|GetBP_MicrowaveTimer)))
  (Variables|Default|SetDoorOpen false)
  (Variables|Default|SetStartButton false)
  (Variables|Default|SetButtonOrginalPosition (Transformation|GetWorldLocation (Variables|Default|GetButton)))
  (Variables|Default|SetPointHandleOrignalRotate (Transformation|GetWorldRotation (Variables|Default|GetBP_MicrowaveTimerHandPoint))))

(event EventTick
  (params (DeltaSeconds :type Float%20%28single-precision%29))
  (Utilities|FlowControl|Gate true
    (:Exit
      (if (Variables|Default|GetDoorController)
        (Variables|Default|SetNewDoorRotate (Transformation|GetWorldRotation (Variables|Default|GetDoorPivot)))
        (Variables|Default|SetCurrentAngle (CallFunction|GetDoorAngle))
        (if (< (Math|Float|Absolute(Float) (Variables|Default|GetCurrentAngle)) 8e+01)
          (if (< (Math|Float|Absolute(Float) (- (.yaw (Variables|Default|GetNewDoorRotate)) (.yaw (Variables|Default|GetDoorRotate)))) 2.0)
            (Variables|Default|SetDoorOpen false)
            (else
              (Variables|Default|SetDoorOpen true)))
          (Rendering|SetVisibility (Variables|Default|GetPointLight) (Variables|Default|GetDoorOpen) false)
          (|DoorControll))
        (elif (Variables|Default|GetTimerController)
          (Variables|Default|SetTimerNewRotate (Variables|/Script/Engine.SceneComponent|GetRelativeRotation (Variables|Default|GetBP_MicrowaveTimer)))
          (if (> (.roll (Variables|Default|GetTimerHandRotate)) 0.0)
            (Transformation|SetRelativeRotation (Variables|Default|GetBP_MicrowaveTimer) (Math|Rotator|MakeRotator (.roll (Variables|Default|GetTimerHandRotate)) 0.0 0.0) false false)
            (if (> (- (.roll (Variables|Default|GetTimerNewRotate)) (.roll (Variables|Default|GetTimerRotate))) 2.0) :!label _label
              (if (not (Variables|Default|GetDoorOpen))
                (if (Variables|Default|GetStartButton)
                  (Rendering|SetVisibility (Variables|Default|GetPointLight) true false)
                  (Transformation|AddRelativeRotation (Variables|Default|GetBP_MicrowaveTimer) (Math|Rotator|MakeRotator -0.5 0.0 0.0) false false)
                  (Variables|Default|SetTimerNewRotate (Variables|/Script/Engine.SceneComponent|GetRelativeRotation (Variables|Default|GetBP_MicrowaveTimer)))
                  (Transformation|AddRelativeRotation (Variables|Default|GetPlate) (Math|Rotator|MakeRotator 0.0 0.0 3.0) false false)
                  (Transformation|SetRelativeRotation (Variables|Default|GetBP_MicrowaveTimerHandPoint) (Variables|Default|GetTimerNewRotate) false false)
                  (Utilities|FlowControl|Delay 0.1)
                  (goto _label)))
              (else
                (Rendering|SetVisibility (Variables|Default|GetPointLight) false false)
                (Transformation|SetWorldLocation (Variables|Default|GetButton) (Variables|Default|GetButtonOrginalPosition) false false)
                (Variables|Default|SetStartButton false)))))))))

(fn ConstructionScript)

(fn GetDoorRotation
  (params (OptionalDirection :type Vector) (UseDirection :type Boolean))
  (return (Class|KismetMathLibrary|MakeRotfromYZ (Math|Vector|SelectVector OptionalDirection (CallFunction|GetHandDoorDirection) UseDirection) (Math|Vector|GetUpVector (Variables|Default|GetDoorPivot)))))

(fn GetHandDoorDirection
  (bind _doorpivot (Variables|Default|GetDoorPivot))
  (bind _handposition (Variables|Default|GetHandPosition))
  (bind _returnvalue (Transformation|GetWorldLocation _doorpivot))
  (bind _returnvalue_2 (- _handposition _returnvalue))
  (bind (_x _y) (Math|Vector|BreakVector _returnvalue_2))
  (return (Math|Vector|Normalize (Math|Vector|MakeVector _x _y 0.0))))

(fn GetDoorAngle
  (return (* (Class|KismetMathLibrary|DegAcos (Math|Vector|DotProduct (CallFunction|GetHandDoorDirection) (Variables|Default|GetInitDoorDirection))) (Math|Float|SelectFloat -1.0 1.0 (< (.z (Math|Vector|CrossProduct (CallFunction|GetHandDoorDirection) (Variables|Default|GetInitDoorDirection))) 0.0)))))