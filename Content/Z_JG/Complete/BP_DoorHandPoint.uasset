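; Grabbable hand point used as a child actor of BP_Door, passing the position of the grabbing hand to the door.
; Pickup attaches it to the supplied component, enables tick and opens a gate that calls StartTracking and updates the door's HandPosition from the sphere each frame.
; Drop snaps the sphere back to the last grip location, reattaches to that parent grip, stops door tracking and disables tick.
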(event EventBeginPlay
  (Variables|Default|SetGrip (Class|Actor|GetParentComponent))
  (bind _output_get (Variables|Default|SetDoorHandPointLocation (Transformation|GetWorldLocation (Variables|Default|GetGrip))))
  (Variables|Default|SetNewDoorHandPointLocation _output_get))

(event EventTick
  (params (DeltaSeconds :type Float%20%28single-precision%29))
  (Utilities|FlowControl|Gate true
    (:Exit
      (Variables|Default|SetDoorHandPointLocation (Transformation|GetWorldLocation (Variables|Default|GetGrip)))
      (Variables|Default|SetNewDoorHandPointLocation (Transformation|GetWorldLocation (Variables|Default|GetSphere)))
      (CallFunction|Turnon))))

(event EventPickup
  (params (AttachTo :type Scene%20Component%20Object%20Reference))
  (Actor|Tick|SetActorTickEnabled true)
  (Transformation|AttachComponentToComponent (VehicleSound|GetRootComponent) AttachTo "None" "KeepWorld" "KeepWorld" "KeepWorld" false)
  (Utilities|FlowControl|Gate true) ; enters at Open
)

(event EventDrop
  (Actor|Tick|SetActorTickEnabled false)
  (Transformation|SetWorldLocation (Variables|Default|GetSphere) (Variables|Default|GetDoorHandPointLocation) false false)
  (Transformation|DetachFromActor "KeepWorld" "KeepWorld" "KeepWorld")
  (Transformation|AttachComponentToComponent (VehicleSound|GetRootComponent) (Variables|Default|GetGrip) "None" "KeepWorld" "KeepWorld" "KeepWorld" false)
  (CallFunction|TurnOff)
  (Utilities|FlowControl|Gate true) ; enters at Close
)

(fn ConstructionScript)

(fn Turnon
  (bind _asbp_door (Utilities|Casting|CastToBP_Door (Actor|GetParentActor)))
  (Default|StartTracking _asbp_door)
  (Variables|/Game/Z_JG/Complete/BP_Door.BP_Door_C|SetHandPosition _asbp_door (Variables|Default|GetNewDoorHandPointLocation)))

(fn TurnOff
  (bind _asbp_door (Utilities|Casting|CastToBP_Door (Actor|GetParentActor)))
  (Default|StopTracking _asbp_door)
  (Variables|/Game/Z_JG/Complete/BP_Door.BP_Door_C|SetHandPosition _asbp_door (Variables|Default|GetNewDoorHandPointLocation)))