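; Right-hand drawer door Blueprint that swings on DoorPivot to follow a hand position while tracking is active.
; StartTracking and StopTracking toggle actor tick and a gate around the rotation update.
; Each tick measures the hand's signed horizontal angle from the pivot's initial right vector, using dot and cross products.
; Angles within 88 degrees either way select a minimum-limit, maximum-limit or hand-following rotation for the pivot.
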(event Custom|StopTracking
  (Actor|Tick|SetActorTickEnabled false)
  (Utilities|FlowControl|Gate true) ; enters at Close
)

(event Custom|StartTracking
  (Actor|Tick|SetActorTickEnabled true)
  (Utilities|FlowControl|Gate true) ; enters at Open
)

(event EventBeginPlay
  (Variables|Default|SetInitDoorDirection (Math|Vector|GetRightVector (Variables|Default|GetDoorPivot))))

(event EventTick
  (params (DeltaSeconds :type Float%20%28single-precision%29))
  (Utilities|FlowControl|Gate true
    (:Exit
      (Variables|Default|SetCurrentAngle (CallFunction|GetDoorAngle))
      (if (< (Math|Float|Absolute(Float) (Variables|Default|GetCurrentAngle)) 88.0)
        (if (<= (Variables|Default|GetCurrentAngle) (Variables|Default|GetMinAngle))
          (Transformation|SetWorldRotation (Variables|Default|GetDoorPivot) (|GetMinAngleRotation) false false)
          (elif (>= (Variables|Default|GetCurrentAngle) (Variables|Default|GetMaxAngle))
            (Transformation|SetWorldRotation (Variables|Default|GetDoorPivot) (|GetMaxAngleRotation) false false)
            (else
              (Transformation|SetWorldRotation (Variables|Default|GetDoorPivot) (|GetRotation) false false))))))))

(fn ConstructionScript)

(fn GetDoorRotation
  (params (OptionalDirection :type Vector) (UseDirection :type Boolean))
  (return (Class|KismetMathLibrary|MakeRotfromYZ (Math|Vector|SelectVector OptionalDirection (CallFunction|GetHandDoorDirection) UseDirection) (Math|Vector|GetUpVector (Variables|Default|GetDoorPivot)))))

(fn GetHandDoorDirection
  (bind _doorpivot (Variables|Default|GetDoorPivot))
  (bind _handposition (Variables|Default|GetHandPosition))
  (bind _returnvalue (Transformation|GetWorldLocation _doorpivot))
  (bind _returnvalue_2 (- _handposition _returnvalue))
  (bind (_x _y) (Math|Vector|BreakVector _returnvalue_2))
  (return (Math|Vector|Normalize (Math|Vector|MakeVector _x _y 0.0))))

(fn GetDoorAngle
  (return (* (Class|KismetMathLibrary|DegAcos (Math|Vector|DotProduct (CallFunction|GetHandDoorDirection) (Variables|Default|GetInitDoorDirection))) (Math|Float|SelectFloat -1.0 1.0 (< (.z (Math|Vector|CrossProduct (CallFunction|GetHandDoorDirection) (Variables|Default|GetInitDoorDirection))) 0.0)))))