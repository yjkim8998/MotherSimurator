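; Grabbable door handle that feeds the grabbing hand's movement to its parent BP_BaseFurnituerHandPoint actor.
; Pickup attaches the handle to the grabbing component, enables Tick and opens a gate that sends the Sphere's world position and rotation to the parent each frame.
; Drop moves the Sphere back to the Grip's last sampled location, reattaches it to the Grip, stops the parent and closes the gate.
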(event EventBeginPlay
  (Variables|Default|SetGrip (Class|Actor|GetParentComponent))
  (bind _output_get (Variables|Default|SetDoor_HandPointLocation (Transformation|GetWorldLocation (Variables|Default|GetGrip))))
  (Variables|Default|SetDoor_HandPointNewLocation _output_get)
  (bind _output_get_2 (Variables|Default|SetDoor_HandPointRotate (Transformation|GetWorldRotation (Variables|Default|GetGrip))))
  (Variables|Default|SetDoor_HandPointNewRotate _output_get_2))

(event EventTick
  (params (DeltaSeconds :type Float%20%28single-precision%29))
  (Utilities|FlowControl|Gate true
    (:Exit
      (Variables|Default|SetDoor_HandPointLocation (Transformation|GetWorldLocation (Variables|Default|GetGrip)))
      (Variables|Default|SetDoor_HandPointNewLocation (Transformation|GetWorldLocation (Variables|Default|GetSphere)))
      (Variables|Default|SetDoor_HandPointRotate (Transformation|GetWorldRotation (Variables|Default|GetGrip)))
      (Variables|Default|SetDoor_HandPointNewRotate (Transformation|GetWorldRotation (Variables|Default|GetSphere)))
      (CallFunction|TurnonPoint))))

(event EventPickup
  (params (AttachTo :type Scene%20Component%20Object%20Reference))
  (Actor|Tick|SetActorTickEnabled true)
  (Transformation|AttachComponentToComponent (VehicleSound|GetRootComponent) AttachTo "None" "KeepWorld" "KeepWorld" "KeepWorld" false)
  (Utilities|FlowControl|Gate true) ; enters at Open
)

(event EventDrop
  (Actor|Tick|SetActorTickEnabled false)
  (Transformation|SetWorldLocation (Variables|Default|GetSphere) (Variables|Default|GetDoor_HandPointLocation) false false)
  (Transformation|DetachFromActor "KeepWorld" "KeepWorld" "KeepWorld")
  (Transformation|AttachComponentToComponent (VehicleSound|GetRootComponent) (Variables|Default|GetGrip) "None" "KeepWorld" "KeepWorld" "KeepWorld" false)
  (CallFunction|TurnOffPoint)
  (Utilities|FlowControl|Gate true) ; enters at Close
)

(fn ConstructionScript)

(fn TurnonPoint
  (bind _asbp_base_furnituer_hand_point (Utilities|Casting|CastToBP_BaseFurnituerHandPoint (Actor|GetParentActor))
    (:then
      (Default|Start _asbp_base_furnituer_hand_point)
      (Variables|/Game/Z_JG/Complete/BP_BaseFurnituerHandPoint.BP_BaseFurnituerHandPoint_C|SetHandPosition _asbp_base_furnituer_hand_point (Variables|Default|GetDoor_HandPointNewLocation))
      (Variables|/Game/Z_JG/Complete/BP_BaseFurnituerHandPoint.BP_BaseFurnituerHandPoint_C|SetHandRotation _asbp_base_furnituer_hand_point (Variables|Default|GetDoor_HandPointNewRotate)))
    (:CastFailed
      (Development|PrintString "Error BaseDoorHandle.TurnOffPoint"))))

(fn TurnOffPoint
  (bind _asbp_base_furnituer_hand_point (Utilities|Casting|CastToBP_BaseFurnituerHandPoint (Actor|GetParentActor))
    (:then
      (Default|Stop _asbp_base_furnituer_hand_point)
      (Variables|/Game/Z_JG/Complete/BP_BaseFurnituerHandPoint.BP_BaseFurnituerHandPoint_C|SetHandPosition _asbp_base_furnituer_hand_point (Variables|Default|GetDoor_HandPointNewLocation))
      (Variables|/Game/Z_JG/Complete/BP_BaseFurnituerHandPoint.BP_BaseFurnituerHandPoint_C|SetHandRotation _asbp_base_furnituer_hand_point (Variables|Default|GetDoor_HandPointNewRotate)))
    (:CastFailed
      (Development|PrintString "Error BaseDoorHandle.TurnOffPoint"))))