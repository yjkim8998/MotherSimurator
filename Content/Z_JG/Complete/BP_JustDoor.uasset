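; Hinged door Blueprint that follows a tracked hand position, with a handle that must be pushed down before the door opens.
; StartTracking and StopTracking gate the Tick logic; stopping also resets the handle.
; Downward hand offset rolls the handle, and enough roll releases the latch.
; The pivot then turns toward the hand's signed angle, clamped between min and max, and a yaw check re-latches it.
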(event Custom|StopTracking
  (Actor|Tick|SetActorTickEnabled false)
  (Transformation|SetRelativeRotation (Variables|Default|GetDoorHandle) (Variables|Default|GetDoorHandleRotate) false false)
  (Utilities|FlowControl|Gate true) ; enters at Close
)

(event Custom|StartTracking
  (Actor|Tick|SetActorTickEnabled true)
  (Utilities|FlowControl|Gate true) ; enters at Open
)

(event EventBeginPlay
  (Variables|Default|SetInitDoorDirection (Math|Vector|GetRightVector (Variables|Default|GetDoorPivot)))
  (Variables|Default|SetDoorHandleRotate (Variables|/Script/Engine.SceneComponent|GetRelativeRotation (Variables|Default|GetDoorHandle)))
  (Variables|Default|SetHoldHandPosition (Transformation|GetWorldLocation (Variables|Default|GetBP_testdoorhandle)))
  (Variables|Default|SetDoorRotate (Transformation|GetWorldRotation (Variables|Default|GetDoor)))
  (Variables|Default|SetDoorClose true))

(event EventTick
  (params (DeltaSeconds :type Float%20%28single-precision%29))
  (Utilities|FlowControl|Gate true
    (:Exit
      (Variables|Default|SetCurrentAngle (CallFunction|GetDoorAngle))
      (Variables|Default|SetNewDoorHandleRotate (Variables|/Script/Engine.SceneComponent|GetRelativeRotation (Variables|Default|GetDoorHandle)))
      (Variables|Default|SetNewDoorRotate (Transformation|GetWorldRotation (Variables|Default|GetDoor)))
      (if (CallFunction|ShouldHandleRotation)
        (Transformation|SetRelativeRotation (Variables|Default|GetDoorHandle) (Math|Rotator|MakeRotator (* (CallFunction|GetHandleOffset) -3.0) 0.0 0.0) false false))
      (if (Variables|Default|GetDoorClose)
        (if (CallFunction|ShouldDoorOpen)
          (Variables|Default|SetDoorClose false)
          (if (<= (Variables|Default|GetCurrentAngle) (Variables|Default|GetMinAngle)) :!label _label
            ;[1 1 1] 문 닫히는 범위
            (Transformation|SetWorldRotation (Variables|Default|GetDoorPivot) (|GetMinAngleRotation) false false)
            (|SetDoorClose)
            (elif (>= (Variables|Default|GetCurrentAngle) (Variables|Default|GetMaxAngle))
              ;[1 1 1] 열리는 범위
              (Transformation|SetWorldRotation (Variables|Default|GetDoorPivot) (|GetMaxAngleRotation) false false)
              (|SetDoorClose_2)
              (else
                ;[1 1 1] 중간 덜렁거리는 상태
                (Transformation|SetWorldRotation (Variables|Default|GetDoorPivot) (|GetRotation) false false)
                (|SetDoorClose_3)))))
        (else
          (goto _label))))))

(fn ConstructionScript)

(fn GetDoorRotation
  (params (OptionalDirection :type Vector) (UseDirection :type Boolean))
  (return (Class|KismetMathLibrary|MakeRotfromYZ (Math|Vector|SelectVector OptionalDirection (CallFunction|GetHandDoorDirection) UseDirection) (Math|Vector|GetUpVector (Variables|Default|GetDoorPivot)))))

(fn GetHandDoorDirection
  (bind _doorpivot (Variables|Default|GetDoorPivot))
  (bind _handposition (Variables|Default|GetHandPosition))
  (bind _returnvalue (Transformation|GetWorldLocation _doorpivot))
  (bind _returnvalue_2 (- _handposition _returnvalue))
  (bind (_x _y) (Math|Vector|BreakVector _returnvalue_2))
  (return (Math|Vector|Normalize (Math|Vector|MakeVector _x _y 0.0))))

(fn GetDoorAngle
  (return (* (Class|KismetMathLibrary|DegAcos (Math|Vector|DotProduct (CallFunction|GetHandDoorDirection) (Variables|Default|GetInitDoorDirection))) (Math|Float|SelectFloat -1.0 1.0 (< (.z (Math|Vector|CrossProduct (CallFunction|GetHandDoorDirection) (Variables|Default|GetInitDoorDirection))) 0.0)))))

(fn ShouldHandleRotation
  (bind _returnvalue (CallFunction|GetHandleOffset))
  (return (and (<= _returnvalue 15.0) (>= _returnvalue 0.0))))

(fn GetHandleOffset
  (return (- (.z (Variables|Default|GetHoldHandPosition)) (.z (Variables|Default|GetHandPosition)))))

(fn ShouldDoorOpen
  (return (>= (- (.roll (Variables|Default|GetDoorHandleRotate)) (.roll (Variables|Default|GetNewDoorHandleRotate))) 3e+01)))

(fn ShouldDoorClose
  (return (< (+ (.yaw (Variables|Default|GetNewDoorRotate)) 1.8e+02) 3.0)))