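; BP_Oven_c is a VR oven that a motion controller switches on and off by touching its button while the child-actor door is closed.
; Toggling shifts the button and sets the point light's visibility.
; While on and closed, it runs a one-second delayed loop that calls Cooking on food in the trigger whose cook types match the oven's, set in the construction script.
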(event OnComponentBeginOverlap(ButtonUp)
  (params (OverlappedComponent :type Primitive%20Component%20Object%20Reference) (OtherActor :type Actor%20Object%20Reference) (OtherComp :type Primitive%20Component%20Object%20Reference) (OtherBodyIndex :type Integer) (bFromSweep :type Boolean) (SweepResult :type Hit%20Result%20Structure%20%28by%20ref%29))
  (bind _asbp_oven_door (Utilities|Casting|CastToBP_OvenDoor (Variables|/Script/Engine.ChildActorComponent|GetChildActor (Variables|Default|GetOven_Door))))
  (if (not (Variables|/Game/Z_JG/BP_OvenDoor.BP_OvenDoor_C|GetDoorOpen _asbp_oven_door))
    (Utilities|Casting|CastToBP_MotionController OtherActor)
    (if (Variables|Default|GetButtonOn)
      (CallFunction|OvenOff)
      (else
        (CallFunction|Ovenon)))
    (if (not (Variables|/Game/Z_JG/BP_OvenDoor.BP_OvenDoor_C|GetDoorOpen _asbp_oven_door)) :!label _label
      (if (Variables|Default|GetButtonOn)
        (Utilities|FlowControl|Delay 1.0)
        (|CheckCooking_Oven
          (:True
            (goto _label))
          (:False
            (goto _label)))))))

(event Custom|OvenOff
  (Transformation|AddRelativeLocation (Variables|Default|GetButton) "0,4.500000,0.000000" false false)
  (bind _output_get (Variables|Default|SetButtonOn false))
  (Rendering|SetVisibility (Variables|Default|GetPointLight) _output_get false))

(event Custom|OvenOn
  (Transformation|AddRelativeLocation (Variables|Default|GetButton) "0,-4.500000,0.000000" false false)
  (bind _output_get (Variables|Default|SetButtonOn true))
  (Rendering|SetVisibility (Variables|Default|GetPointLight) _output_get false))

(event EventBeginPlay
  (Variables|Default|SetButtonOn false))

(event EventOff
  (Variables|Default|SetButtonOn false))

(fn ConstructionScript
  (Variables|Default|SetCookType_tool "NewEnumerator2"))