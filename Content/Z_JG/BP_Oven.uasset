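; BP_Oven is an oven actor whose hinged door follows a tracked hand position.
; BeginPlay records the door's initial direction and uses actor yaw to choose the hinge plane and angle limits.
; StartTracking and StopTracking toggle Tick and a Gate.
; While tracking, Tick finds the signed door angle from the hand direction projected onto that plane, then sets the pivot rotation via minimum, maximum or free-rotation helpers.
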(event Custom|StopTracking
  (Actor|Tick|SetActorTickEnabled false)
  (Utilities|FlowControl|Gate true) ; enters at Close
)

(event Custom|StartTracking
  (Actor|Tick|SetActorTickEnabled true)
  (Utilities|FlowControl|Gate true) ; enters at Open
)

(event EventBeginPlay
  (bind _defaultsceneroot (Variables|Default|GetDefaultSceneRoot))
  (bind _defaultsceneroot_2 (Variables|Default|GetDefaultSceneRoot))
  (bind _returnvalue (Transformation|GetWorldRotation _defaultsceneroot))
  (bind _returnvalue_2 (Transformation|GetWorldRotation _defaultsceneroot_2))
  (bind _returnvalue_3 (Math|Float|Absolute(Float) (.yaw _returnvalue_2)))
  (bind _returnvalue_4 (Math|Float|Absolute(Float) (.yaw _returnvalue)))
  (Variables|Default|SetInitOvenDoorDirection (Math|Vector|GetUpVector (Variables|Default|GetDoorPivot)))
  (Variables|Default|SetSetRotate90 (or (and (>= _returnvalue_4 89.0) (<= _returnvalue_4 91.0)) (and (>= _returnvalue_3 269.0) (<= _returnvalue_3 271.0))))
  (if (or (>= (Math|Float|Absolute(Float) (.yaw (Transformation|GetWorldRotation (Variables|Default|GetDefaultSceneRoot)))) 179.0) (>= -89.0 (.yaw (Transformation|GetWorldRotation (Variables|Default|GetDefaultSceneRoot)))))
    (Variables|Default|SetMinAngle -9e+01)
    (Variables|Default|SetMaxAngle 0.0)))

(event EventTick
  (params (DeltaSeconds :type Float%20%28single-precision%29))
  (Utilities|FlowControl|Gate true
    (:Exit
      (Variables|Default|SetCurrentAngle (CallFunction|GetDoorAngle))
      (if (< (Math|Float|Absolute(Float) (Variables|Default|GetCurrentAngle)) 8e+01)
        (if (<= (Variables|Default|GetCurrentAngle) (Variables|Default|GetMinAngle))
          (Transformation|SetWorldRotation (Variables|Default|GetDoorPivot) (|GetMinAngleRotation) false false)
          (elif (>= (Variables|Default|GetCurrentAngle) (Variables|Default|GetMaxAngle))
            (Transformation|SetWorldRotation (Variables|Default|GetDoorPivot) (|GetMaxAngleRotation) false false)
            (else
              (Transformation|SetWorldRotation (Variables|Default|GetDoorPivot) (|GetRotation) false false))))))))

(fn ConstructionScript)

(fn GetOvenDoorRotation
  (params (OptionalDirection :type Vector) (UseDirection :type Boolean))
  (bind _returnvalue (CallFunction|GetHandDoorDirection))
  (bind _doorpivot (Variables|Default|GetDoorPivot))
  (bind _returnvalue_2 (Math|Vector|SelectVector OptionalDirection _returnvalue UseDirection))
  (return (Math|Rotator|SelectRotator (Math|Rotator|MakeRotfromZX _returnvalue_2 (Math|Vector|GetForwardVector _doorpivot)) (Math|Rotator|MakeRotfromZY _returnvalue_2 (Math|Vector|GetRightVector _doorpivot)) (Variables|Default|GetSetRotate90))))

(fn GetHandDoorDirection
  (bind _handposition (Variables|Default|GetHandPosition))
  (bind _doorpivot (Variables|Default|GetDoorPivot))
  (bind _returnvalue (Transformation|GetWorldLocation _doorpivot))
  (bind _returnvalue_2 (- _handposition _returnvalue))
  (bind (_x _y _z) (Math|Vector|BreakVector _returnvalue_2))
  (bind (_x_2 _y_2 _z_2) (Math|Vector|BreakVector _returnvalue_2))
  (return (Math|Vector|Normalize (Math|Vector|SelectVector (Math|Vector|MakeVector _x_2 0.0 _z_2) (Math|Vector|MakeVector 0.0 _y _z) (Variables|Default|GetSetRotate90)))))

(fn GetDoorAngle
  (bind _returnvalue (CallFunction|GetHandDoorDirection))
  (bind _initovendoordirection (Variables|Default|GetInitOvenDoorDirection))
  (bind _returnvalue_2 (Math|Vector|CrossProduct _returnvalue _initovendoordirection))
  (return (* (Class|KismetMathLibrary|DegAcos (Math|Vector|DotProduct (CallFunction|GetHandDoorDirection) (Variables|Default|GetInitOvenDoorDirection))) (Math|Float|SelectFloat -1.0 1.0 (< (Math|Float|SelectFloat (.y _returnvalue_2) (.x _returnvalue_2) (Variables|Default|GetSetRotate90)) 0.0)))))