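; Grabbable handle for a left test door, run as a child actor that feeds hand position to its parent BP_testdoor_left.
; Pickup attaches the handle to the grabber and opens a Tick gate, which each frame passes the Sphere's location to the door as HandPosition and calls StartTracking.
; Drop snaps the Sphere to the last stored Grip location, reattaches the handle to the Grip and stops door tracking.
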(event EventBeginPlay
  (Variables|Default|SetGrip (Class|Actor|GetParentComponent))
  (bind _output_get (Variables|Default|SetDoorHandPointLocation (Transformation|GetWorldLocation (Variables|Default|GetGrip))))
  (Variables|Default|SetNewDoorHandPointLocation _output_get))

(event EventTick
  (params (DeltaSeconds :type Float%20%28single-precision%29))
  (Utilities|FlowControl|Gate true
    (:Exit
      (Variables|Default|SetDoorHandPointLocation (Transformation|GetWorldLocation (Variables|Default|GetGrip)))
      (Variables|Default|SetNewDoorHandPointLocation (Transformation|GetWorldLocation (Variables|Default|GetSphere)))
      (CallFunction|Turnon))))

(event EventPickup
  (params (AttachTo :type Scene%20Component%20Object%20Reference))
  (Actor|Tick|SetActorTickEnabled true)
  (Transformation|AttachComponentToComponent (VehicleSound|GetRootComponent) AttachTo "None" "KeepWorld" "KeepWorld" "KeepWorld" false)
  (Utilities|FlowControl|Gate true) ; enters at Open
)

(event EventDrop
  (Actor|Tick|SetActorTickEnabled false)
  (Transformation|SetWorldLocation (Variables|Default|GetSphere) (Variables|Default|GetDoorHandPointLocation) false false)
  (Transformation|DetachFromActor "KeepWorld" "KeepWorld" "KeepWorld")
  (Transformation|AttachComponentToComponent (VehicleSound|GetRootComponent) (Variables|Default|GetGrip) "None" "KeepWorld" "KeepWorld" "KeepWorld" false)
  (CallFunction|TurnOff)
  (Utilities|FlowControl|Gate true) ; enters at Close
)

(fn ConstructionScript)

(fn Turnon
  (bind _asbp_testdoor_left (Utilities|Casting|CastToBP_testdoor_left (Actor|GetParentActor))
    (:then
      (Default|StartTracking _asbp_testdoor_left)
      (Variables|/Game/Z_JG/base_test/BP_testdoor_left.BP_testdoor_left_C|SetHandPosition _asbp_testdoor_left (Variables|Default|GetNewDoorHandPointLocation)))
    (:CastFailed
      (Development|PrintString "BP_testdoorhandle_new.TrunOn is something worng" true true "(R=0.000000,G=0.660000,B=1.000000,A=1.000000)" 3e+01))))

(fn TurnOff
  (bind _asbp_testdoor_left (Utilities|Casting|CastToBP_testdoor_left (Actor|GetParentActor))
    (:then
      (Default|StopTracking _asbp_testdoor_left)
      (Variables|/Game/Z_JG/base_test/BP_testdoor_left.BP_testdoor_left_C|SetHandPosition _asbp_testdoor_left (Variables|Default|GetNewDoorHandPointLocation)))
    (:CastFailed
      (Development|PrintString "BP_testdoorhandle_new.TrunOff is something worng" true true "(R=0.000000,G=0.660000,B=1.000000,A=1.000000)" 3e+01))))