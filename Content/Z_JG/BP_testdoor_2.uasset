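; Test door Blueprint with a latch handle that follows the vertical movement of a hand and a physics-driven swing.
; DoorOn and DoorOff toggle Tick and a gate, during which the downward offset between GripO's initial location and externally supplied NewHandLocation pitches the handle.
; Within that offset range, sufficient handle pitch unlatches the door, enabling physics simulation until its yaw returns near closed and physics is switched off again.
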(event Custom|DoorOff
  (Actor|Tick|SetActorTickEnabled false)
  (Transformation|SetRelativeRotation (Variables|Default|GetDoorHandle) (Math|Rotator|MakeRotator 0.0 0.0 -9e+01) false false)
  (Utilities|FlowControl|Gate true) ; enters at Close
)

(event Custom|DoorOn
  (Actor|Tick|SetActorTickEnabled true)
  (Utilities|FlowControl|Gate true) ; enters at Open
)

(event EventBeginPlay
  (Variables|Default|SetDoorRotate (Variables|/Script/Engine.SceneComponent|GetRelativeRotation (Variables|Default|GetDoor)))
  (Variables|Default|SetDoorHandleRotate (Transformation|GetWorldRotation (Variables|Default|GetDoorHandle)))
  (Variables|Default|SetHandLocation (Transformation|GetWorldLocation (Variables|Default|GetGrip_O)))
  (Variables|Default|SetDoorClose true))

(event EventTick
  (params (DeltaSeconds :type Float%20%28single-precision%29))
  (Development|PrintString (Utilities|String|ToString(Float) (- (.x (Variables|Default|GetHandLocation)) (.x (Variables|Default|GetNewHandLocation)))))
  (Utilities|FlowControl|Gate true
    (:Exit
      (Variables|Default|SetNewDoorRotate (Variables|/Script/Engine.SceneComponent|GetRelativeRotation (Variables|Default|GetDoor)))
      (Variables|Default|SetNewDoorHandleRotate (Transformation|GetWorldRotation (Variables|Default|GetDoorHandle)))
      (if (CallFunction|ShouldHandleRotation)
        (Transformation|SetRelativeRotation (Variables|Default|GetDoorHandle) (Math|Rotator|MakeRotator 0.0 (* (CallFunction|GetHandleOffset) 3.0) -9e+01) false false)
        (if (Variables|Default|GetDoorClose)
          (Physics|SetSimulatePhysics (Variables|Default|GetDoor) false)
          (if (CallFunction|ShouldOpenDoor)
            (Variables|Default|SetDoorClose false))
          (else
            (Physics|SetSimulatePhysics (Variables|Default|GetDoor) true)
            (if (CallFunction|ShouldCloseDoor)
              (Variables|Default|SetDoorClose true))))))))

(fn ConstructionScript)

(fn ShouldCloseDoor
  (return (<= (- 1.8e+02 (.yaw (Variables|Default|GetNewDoorRotate))) (Variables|Default|GetCloseDoorOffset))))

(fn ShouldOpenDoor
  (return (>= (- (.pitch (Variables|Default|GetNewDoorHandleRotate)) (.pitch (Variables|Default|GetDoorHandleRotate))) 3e+01)))

(fn ShouldHandleRotation
  (bind _returnvalue (CallFunction|GetHandleOffset))
  (return (and (<= _returnvalue 15.0) (>= _returnvalue 0.0))))

(fn GetHandleOffset
  (return (- (.z (Variables|Default|GetHandLocation)) (.z (Variables|Default|GetNewHandLocation)))))

(fn ShouldDoorOpenMax
  (bind _doorrotate (Variables|Default|GetDoorRotate))
  (return (and (<= (.yaw _doorrotate) (Variables|Default|GetDoorRotateMax)) (>= (.yaw _doorrotate) (Variables|Default|GetDoorRotateMin)))))