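; Test drawer actor that slides along the handle's forward axis while a hand holds it.
; Pickup stores the hand and opens a Tick gate; Drop closes it and clears the hand.
; Each tick projects the hand onto that axis in actor space, then backs off by the handle-to-drawer distance cached at BeginPlay.
; The drawer moves only while its signed offset from the start stays within min/max limits; exceeding them releases it automatically.
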(event Custom|StopTracking
  (Utilities|FlowControl|Gate true) ; enters at Close
)

(event Custom|StartTracking
  (Utilities|FlowControl|Gate true) ; enters at Open
)

(event EventBeginPlay
  (Variables|Default|SetHandleOffset (CallFunction|GetHandleOffset))
  (Variables|Default|SetDrawerInitLocation (Transformation|GetWorldLocation (Variables|Default|GetDrawers))))

(event EventTick
  (params (DeltaSeconds :type Float%20%28single-precision%29))
  (Utilities|FlowControl|Gate true
    (:Exit
      (Variables|Default|SetNewDrawerLocation (CallFunction|GetDrawerNewLocation))
      (if (CallFunction|ShouldUpdateDrawer)
        (Transformation|SetWorldLocation (Variables|Default|GetDrawers) (Variables|Default|GetNewDrawerLocation) false false)
        (else
          (CallFunction|Drop))))))

(event EventPickup
  (params (AttachTo :type Scene%20Component%20Object%20Reference))
  (Variables|컴포넌트|SetHand AttachTo)
  (CallFunction|StartTracking))

(event EventDrop
  (CallFunction|StopTracking)
  (Variables|컴포넌트|SetHand 0))

(fn ConstructionScript)

(fn GetHandleOffset
  (return (Math|Float|Absolute(Float) (Math|Vector|VectorLength (- (Transformation|GetWorldLocation (Variables|Default|GetHandle)) (Transformation|GetWorldLocation (Variables|Default|GetDrawers)))))))

(fn GetDrawerOffset
  (bind _drawerinitlocation (Variables|Default|GetDrawerInitLocation))
  (bind _newdrawerlocation (Variables|Default|GetNewDrawerLocation))
  (bind _returnvalue (- _newdrawerlocation _drawerinitlocation))
  (return (* (Math|Vector|VectorLength _returnvalue) (Math|Float|SelectFloat -1.0 1.0 (< (Math|Vector|DotProduct (Math|Vector|Normalize _returnvalue) (Math|Vector|GetForwardVector (Transformation|GetWorldRotation (Variables|Default|GetHandle)))) 0.0)))))

(fn GetHandonDrawerForwardVector
  (return (Math|Transform|TransformLocation (Transformation|GetActorTransform) (Math|Vector|ProjectVectorontoVector (Math|Transform|InverseTransformLocation (Transformation|GetActorTransform) (Transformation|GetWorldLocation (Variables|컴포넌트|GetHand))) (Math|Vector|GetForwardVector (Variables|/Script/Engine.SceneComponent|GetRelativeRotation (Variables|Default|GetHandle)))))))

(fn GetDrawerNewLocation
  (return (+ (CallFunction|GetHandonDrawerForwardVector) (* (Math|Vector|NegateVector (Math|Vector|GetForwardVector (Transformation|GetWorldRotation (Variables|Default|GetHandle)))) (Variables|Default|GetHandleOffset)))))

(fn ShouldUpdateDrawer
  (bind _returnvalue (CallFunction|GetDrawerOffset))
  (return (and (>= _returnvalue (Variables|Default|GetMinOffset)) (<= _returnvalue (Variables|Default|GetMaxOffset)))))