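; Test actor for a hand-pulled drawer that slides along one axis while held, with debug prints on pickup and drop.
; Pickup stores the hand component and opens a Tick gate; drop closes it and resets Point to its starting location.
; Each tick projects the hand onto the handle's forward axis in actor space, subtracts the handle offset, and moves Drawers only when the signed travel from its start stays within min/max limits.
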(event Custom|StopTracking
  (Utilities|FlowControl|Gate true) ; enters at Close
)

(event Custom|StartTracking
  (Utilities|FlowControl|Gate true) ; enters at Open
)

(event Custom|CustomEvent
  (params (AttachTo :type Scene%20Component%20Object%20Reference))
  (Development|PrintString (Utilities|GetDisplayName AttachTo) true true "(R=0.000000,G=0.660000,B=1.000000,A=1.000000)" 1e+01)
  (Development|PrintString "Pickup" true true "(R=0.000000,G=0.660000,B=1.000000,A=1.000000)" 1e+01)
  (Variables|Default|SetHand AttachTo)
  (CallFunction|StartTracking))

(event Custom|CustomEvent_1
  (Development|PrintString "Drop" true true "(R=0.000000,G=0.660000,B=1.000000,A=1.000000)" 1e+01)
  (CallFunction|StopTracking)
  (Transformation|SetWorldLocation (Variables|Default|GetPoint) (Variables|Default|GetPointLocation) false false)
  (Variables|Default|SetHand 0))

(event EventBeginPlay
  (Variables|Default|SetHandleOffset (CallFunction|GetHandleOffset))
  (Variables|Default|SetDrawerInitLocation (Transformation|GetWorldLocation (Variables|Default|GetDrawers)))
  (Variables|Default|SetPointLocation (CallFunction|GetHandPoint)))

(event EventTick
  (params (DeltaSeconds :type Float%20%28single-precision%29))
  (Utilities|FlowControl|Gate true
    (:Exit
      (Variables|Default|SetNewDrawerLocation (CallFunction|GetDrawerNewLocation))
      (if (CallFunction|ShouldUpdateDrawer)
        (Transformation|SetWorldLocation (Variables|Default|GetDrawers) (Variables|Default|GetNewDrawerLocation) false false)))))

(fn ConstructionScript)

(fn GetHandleOffset
  (return (Math|Float|Absolute(Float) (Math|Vector|VectorLength (- (Transformation|GetWorldLocation (Variables|Default|GetHandle)) (Transformation|GetWorldLocation (Variables|Default|GetDrawers)))))))

(fn GetDrawerOffset
  (bind _drawerinitlocation (Variables|Default|GetDrawerInitLocation))
  (bind _newdrawerlocation (Variables|Default|GetNewDrawerLocation))
  (bind _returnvalue (- _newdrawerlocation _drawerinitlocation))
  (return (* (Math|Vector|VectorLength _returnvalue) (Math|Float|SelectFloat -1.0 1.0 (< (Math|Vector|DotProduct (Math|Vector|Normalize _returnvalue) (Math|Vector|GetForwardVector (Transformation|GetWorldRotation (Variables|Default|GetHandle)))) 0.0)))))

(fn GetHandonDrawerForwardVector
  (return (Math|Transform|TransformLocation (Transformation|GetActorTransform) (Math|Vector|ProjectVectorontoVector (Math|Transform|InverseTransformLocation (Transformation|GetActorTransform) (Transformation|GetWorldLocation (Variables|Default|GetHand))) (Math|Vector|GetForwardVector (Variables|/Script/Engine.SceneComponent|GetRelativeRotation (Variables|Default|GetHandle)))))))

(fn GetDrawerNewLocation
  (return (+ (CallFunction|GetHandonDrawerForwardVector) (* (Math|Vector|NegateVector (Math|Vector|GetForwardVector (Transformation|GetWorldRotation (Variables|Default|GetHandle)))) (Variables|Default|GetHandleOffset)))))

(fn ShouldUpdateDrawer
  (bind _returnvalue (CallFunction|GetDrawerOffset))
  (return (and (>= _returnvalue (Variables|Default|GetMinOffset)) (<= _returnvalue (Variables|Default|GetMaxOffset)))))

(fn GetHandPoint
  (return (Transformation|GetWorldLocation (Variables|Default|GetPoint))))