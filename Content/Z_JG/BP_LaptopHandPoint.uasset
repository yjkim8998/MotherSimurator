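; Grabbable hand point on BP_Laptop that feeds the position of the holder's hand to the laptop for tracking.
; Pickup attaches it to the grabber and opens a Tick gate that keeps starting tracking and passing the Cube's world location as the laptop's HandPosition.
; Drop moves the Cube back to the saved Grip location, reattaches to Grip, stops tracking and closes the gate.
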(event EventBeginPlay
  (Variables|Default|SetGrip (Class|Actor|GetParentComponent))
  (bind _output_get (Variables|Default|SetScreen_HandPointLocation (Transformation|GetWorldLocation (Variables|Default|GetGrip))))
  (Variables|Default|SetScreen_HandPointNewLocation _output_get))

(event EventTick
  (params (DeltaSeconds :type Float%20%28single-precision%29))
  (Utilities|FlowControl|Gate true
    (:Exit
      (Variables|Default|SetScreen_HandPointLocation (Transformation|GetWorldLocation (Variables|Default|GetGrip)))
      (Variables|Default|SetScreen_HandPointNewLocation (Transformation|GetWorldLocation (Variables|Default|GetCube)))
      (CallFunction|TurnonPoint))))

(event EventPickup
  (params (AttachTo :type Scene%20Component%20Object%20Reference))
  (Actor|Tick|SetActorTickEnabled true)
  (Transformation|AttachComponentToComponent (VehicleSound|GetRootComponent) AttachTo "None" "KeepRelative" "KeepRelative" "KeepRelative" true)
  (Utilities|FlowControl|Gate true) ; enters at Open
)

(event EventDrop
  (Actor|Tick|SetActorTickEnabled false)
  (Transformation|SetWorldLocation (Variables|Default|GetCube) (Variables|Default|GetScreen_HandPointLocation) false false)
  (Transformation|DetachFromActor "KeepRelative" "KeepRelative" "KeepRelative")
  (Transformation|AttachComponentToComponent (VehicleSound|GetRootComponent) (Variables|Default|GetGrip) "None" "KeepRelative" "KeepRelative" "KeepRelative" true)
  (CallFunction|TurnOffPoint)
  (Utilities|FlowControl|Gate true) ; enters at Close
)

(fn ConstructionScript)

(fn TurnonPoint
  (bind _asbp_laptop (Utilities|Casting|CastToBP_Laptop (Actor|GetParentActor)))
  (Default|StartTracking _asbp_laptop)
  (Variables|/Game/Z_JG/BP_Laptop.BP_Laptop_C|SetHandPosition _asbp_laptop (Variables|Default|GetScreen_HandPointNewLocation)))

(fn TurnOffPoint
  (bind _asbp_laptop (Utilities|Casting|CastToBP_Laptop (Actor|GetParentActor)))
  (Default|StopTracking _asbp_laptop)
  (Variables|/Game/Z_JG/BP_Laptop.BP_Laptop_C|SetHandPosition _asbp_laptop (Variables|Default|GetScreen_HandPointNewLocation)))