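; A test drawer actor that keeps sliding with simulated momentum and friction after being let go.
; StartSimulateDrawerPhysics takes an initial velocity and opens a Tick gate, which sets the drawer's relative X from a closed-form constant-deceleration equation, clamped to the drawer length.
; The gate closes once velocity crosses zero or the drawer reaches either end, so no physics body simulation is used.
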(event Custom|StopSimulateDrawerPhysics
  (bind _drawers (Variables|Default|GetDrawers))
  (bind _relativelocation (Variables|/Script/Engine.SceneComponent|GetRelativeLocation _drawers))
  (Development|PrintString "Drop" true true "(R=0.000000,G=0.660000,B=1.000000,A=1.000000)" 1e+01)
  (Utilities|FlowControl|Gate true) ; enters at Close
)

(event Custom|StartSimulateDrawerPhysics
  (params (DrawerInitialVelocity :type Float%20%28single-precision%29))
  (bind _drawers (Variables|Default|GetDrawers))
  (bind _relativelocation (Variables|/Script/Engine.SceneComponent|GetRelativeLocation _drawers))
  (Development|PrintString "PickUp" true true "(R=0.000000,G=0.660000,B=1.000000,A=1.000000)" 1e+01)
  (Variables|Default|SetDrawerInitialVelocity DrawerInitialVelocity)
  (Variables|Default|SetDrawerTimeSinceLetGo 0.0)
  (Utilities|FlowControl|Gate true) ; enters at Open
)

(event EventTick
  (params (DeltaSeconds :type Float%20%28single-precision%29))
  (bind _drawers (Variables|Default|GetDrawers))
  (bind _relativelocation (Variables|/Script/Engine.SceneComponent|GetRelativeLocation _drawers))
  (Utilities|FlowControl|Gate true
    (:Exit
      (Variables|Default|SetDrawerTimeSinceLetGo (+ (Variables|Default|GetDrawerTimeSinceLetGo) DeltaSeconds))
      (Transformation|SetRelativeLocation (Variables|Default|GetDrawers) (Math|Vector|MakeVector (Math|Float|Clamp(Float) (+ (Variables|Default|GetCurrentDrawerPosition) (- (* (Variables|Default|GetDrawerInitialVelocity) (Variables|Default|GetDrawerTimeSinceLetGo)) (* 0.5 (* (Variables|Default|GetDrawerFriction) 9.8e+02) (Math|Float|Square (Variables|Default|GetDrawerTimeSinceLetGo)) (Math|Float|Sign(Float) (Variables|Default|GetDrawerInitialVelocity))))) 0.0 (Variables|Default|GetDrawerLength)) 0.0 0.0) false false)
      (if (Math|Boolean|ORBoolean (select (<= (Variables|Default|GetDrawerInitialVelocity) 0.0) (> (- (Variables|Default|GetDrawerInitialVelocity) (* (* (Variables|Default|GetDrawerFriction) 9.8e+02) (Variables|Default|GetDrawerTimeSinceLetGo) (Math|Float|Sign(Float) (Variables|Default|GetDrawerInitialVelocity)))) 0.0) (<= (- (Variables|Default|GetDrawerInitialVelocity) (* (* (Variables|Default|GetDrawerFriction) 9.8e+02) (Variables|Default|GetDrawerTimeSinceLetGo) (Math|Float|Sign(Float) (Variables|Default|GetDrawerInitialVelocity)))) 0.0)) (Math|Float|NearlyEqual(Float) (.x _relativelocation) 0.0 1e-06) (Math|Float|NearlyEqual(Float) (.x _relativelocation) (Variables|Default|GetDrawerLength) 1e-06))
        (CallFunction|StopSimulateDrawerPhysics)))))

(fn ConstructionScript)