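; Test drawer actor that can be picked up and dropped, with an attempted limit on its travel.
; BeginPlay stores the mesh's world location as an anchor.
; Pickup disables physics, attaches to the given component and runs the distance clamp once, not continuously; Drop restores physics and detaches.
; The clamp sets the location to the scaled offset direction without adding the anchor back.
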(event EventPickup
  (params (AttachTo :type Scene%20Component%20Object%20Reference))
  (Physics|SetSimulatePhysics (Variables|Debug|GetStaticMeshComponent) false)
  (Transformation|AttachComponentToComponent (VehicleSound|GetRootComponent) AttachTo "None" "KeepWorld" "KeepWorld" "KeepWorld" false)
  (CallFunction|LimitMovement (Variables|Default|GetSetDrawerOffset) (Variables|Default|GetMaxOffset)))

(event EventDrop
  (Physics|SetSimulatePhysics (Variables|Debug|GetStaticMeshComponent) true)
  (Transformation|DetachFromActor "KeepRelative" "KeepRelative" "KeepRelative"))

(event EventBeginPlay
  (Variables|Default|SetSetDrawerOffset (Transformation|GetWorldLocation (Variables|Debug|GetStaticMeshComponent))))

(fn ConstructionScript)

(fn LimitMovement
  (params (Anchor%20Position :type Vector) (Anchot%20Distance :type Float%20%28single-precision%29))
  (bind _returnvalue (Transformation|GetActorLocation))
  (bind _returnvalue_2 (- _returnvalue Anchor%20Position))
  (if (> (Math|Vector|VectorLength _returnvalue_2) Anchot%20Distance)
    (Transformation|SetActorLocation (* (Math|Vector|Normalize _returnvalue_2) Anchot%20Distance) false false)))