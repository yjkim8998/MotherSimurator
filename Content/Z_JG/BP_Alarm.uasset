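; BP_Alarm is a grabbable alarm clock actor with a push-button countdown timer.
; Overlapping the button toggles it down or up, starting a looping Delay countdown shown on the Time text or resetting it.
; Reaching zero sets IsSoundOn, though no sound plays in this graph.
; Pickup and Drop handle attachment and clock physics, and switch a Tick gate that drives nothing.
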(event OnComponentBeginOverlap(PushButton)
  (params (OverlappedComponent :type Primitive%20Component%20Object%20Reference) (OtherActor :type Actor%20Object%20Reference) (OtherComp :type Primitive%20Component%20Object%20Reference) (OtherBodyIndex :type Integer) (bFromSweep :type Boolean) (SweepResult :type Hit%20Result%20Structure%20%28by%20ref%29))
  (if (Variables|Default|GetIsButtonOn)
    (Transformation|AddRelativeLocation (Variables|Default|GetButton) "0, 0,22.500000" false false)
    (Variables|Default|SetIsButtonOn false)
    (Variables|Default|SetIsSoundOn false)
    (Variables|Default|SetTimeValue 3e+01 :!label _label)
    (Rendering|Components|TextRender|SetText (Variables|Default|GetTime) (Utilities|Text|ToText(Float) (Variables|Default|GetTimeValue) "HalfToEven"))
    (else
      (Transformation|AddRelativeLocation (Variables|Default|GetButton) "0.000000, 0,-22.500000" false false)
      (Variables|Default|SetIsButtonOn true)
      (if (Variables|Default|GetIsButtonOn) :!label _label_2
        (if (> (Variables|Default|GetTimeValue) 0.0)
          (Rendering|Components|TextRender|SetText (Variables|Default|GetTime) (Utilities|Text|ToText(Float) (Variables|Default|GetTimeValue) "HalfToEven"))
          (Utilities|FlowControl|Delay (Variables|Default|GetDelay))
          (Variables|Default|SetTimeValue (- (Variables|Default|GetTimeValue) (Variables|Default|GetDelay)))
          (goto _label_2)
          (else
            (Rendering|Components|TextRender|SetText (Variables|Default|GetTime) (Utilities|Text|ToText(Float) (Variables|Default|GetTimeValue) "HalfToEven"))
            (Variables|Default|SetIsSoundOn true)))
        (else
          (goto _label))))))

(event Custom|Stop
  (Actor|Tick|SetActorTickEnabled false)
  (Utilities|FlowControl|Gate true) ; enters at Close
)

(event Custom|Start
  (Actor|Tick|SetActorTickEnabled true)
  (Utilities|FlowControl|Gate true) ; enters at Open
)

(event EventBeginPlay
  (Variables|Default|SetIsButtonOn false)
  (Variables|Default|SetTimeValue 3e+01)
  (Variables|Default|SetIsSoundOn false))

(event EventPickup
  (params (AttachTo :type Scene%20Component%20Object%20Reference))
  (Physics|SetSimulatePhysics (Variables|Default|GetClock) false)
  (Transformation|AttachComponentToComponent (VehicleSound|GetRootComponent) AttachTo "None" "KeepWorld" "KeepWorld" "KeepWorld" false)
  (CallFunction|Start))

(event EventTick
  (params (DeltaSeconds :type Float%20%28single-precision%29))
  (Utilities|FlowControl|Gate true))

(event EventDrop
  (Physics|SetSimulatePhysics (Variables|Default|GetClock) true)
  (Transformation|DetachFromActor "KeepWorld" "KeepWorld" "KeepWorld")
  (CallFunction|Stop))

(fn ConstructionScript)