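; Grabbable hand point for the timer on BP_Microwave, used as a child actor of it that responds to Pickup and Drop.
; Pickup attaches it to the grabber and opens a Tick gate that records the Sphere's world rotation, passing it to the microwave with TimerStart every frame.
; Drop snaps the Sphere back to the parent Grip's location, keeps the last rotation, reattaches to Grip and calls TimerStop.
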(event EventBeginPlay
  (Variables|Default|SetGrip (Class|Actor|GetParentComponent))
  (Variables|Default|SetDoor_HandPointLocation (Transformation|GetWorldLocation (Variables|Default|GetGrip)))
  (Variables|Default|SetTimer_HandPointRotate (Variables|/Script/Engine.SceneComponent|GetRelativeRotation (Variables|Default|GetSphere))))

(event EventTick
  (params (DeltaSeconds :type Float%20%28single-precision%29))
  (Utilities|FlowControl|Gate true
    (:Exit
      (Variables|Default|SetDoor_HandPointLocation (Transformation|GetWorldLocation (Variables|Default|GetGrip)))
      (Variables|Default|SetTimer_HandPointNewRotate (Transformation|GetWorldRotation (Variables|Default|GetSphere)))
      (CallFunction|TurnonPoint))))

(event EventPickup
  (params (AttachTo :type Scene%20Component%20Object%20Reference))
  (Actor|Tick|SetActorTickEnabled true)
  (Transformation|AttachComponentToComponent (VehicleSound|GetRootComponent) AttachTo "None" "KeepWorld" "KeepWorld" "KeepWorld" false)
  (Utilities|FlowControl|Gate true) ; enters at Open
)

(event EventDrop
  (Actor|Tick|SetActorTickEnabled false)
  (Transformation|SetWorldLocation (Variables|Default|GetSphere) (Variables|Default|GetDoor_HandPointLocation) false false)
  (Transformation|SetWorldRotation (Variables|Default|GetSphere) (Variables|Default|GetTimer_HandPointNewRotate) false false)
  (Transformation|DetachFromActor "KeepWorld" "KeepWorld" "KeepWorld")
  (Transformation|AttachComponentToComponent (VehicleSound|GetRootComponent) (Variables|Default|GetGrip) "None" "KeepWorld" "KeepWorld" "KeepWorld" false)
  (CallFunction|TurnOffPoint)
  (Utilities|FlowControl|Gate true) ; enters at Close
)

(fn ConstructionScript)

(fn TurnonPoint
  (bind _asbp_microwave (Utilities|Casting|CastToBP_Microwave (Actor|GetParentActor)))
  (Default|TimerStart _asbp_microwave)
  (Variables|/Game/Z_JG/BP_Microwave.BP_Microwave_C|SetTimerHandRotate _asbp_microwave (Variables|Default|GetTimer_HandPointNewRotate)))

(fn TurnOffPoint
  (bind _asbp_microwave (Utilities|Casting|CastToBP_Microwave (Actor|GetParentActor)))
  (Default|TimerStop _asbp_microwave)
  (Variables|/Game/Z_JG/BP_Microwave.BP_Microwave_C|SetTimerHandRotate _asbp_microwave (Variables|Default|GetTimer_HandPointNewRotate)))