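; BP_WaterBottle is a physics bottle that can be picked up, dropped and tilted to pour water.
; Pickup disables physics, attaches the bottle and enables Tick; Drop reverses this and stops the water trail.
; While Tick runs, roll or yaw beyond a threshold starts the WaterFall trail and spawns small BP_WaterCollision actors at it after short delays.
; Hits report a delayed noise event, with loudness from velocity and mass, capped at MaxNoise.
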(event EventBeginPlay
  (Effects|Particles|Trails|EndTrails (Variables|Default|GetWaterFall)))

(event EventPickup
  (params (AttachTo :type Scene%20Component%20Object%20Reference))
  ;[1 1 1] PickUp 이벤트
  (Physics|SetSimulatePhysics (Variables|Default|GetStaticMeshComponent) false)
  (Transformation|AttachComponentToComponent (VehicleSound|GetRootComponent) AttachTo "None" "KeepWorld" "KeepWorld" "KeepWorld" false)
  (Actor|Tick|SetActorTickEnabled true))

(event Collision|EventHit
  (params (MyComp :type Primitive%20Component%20Object%20Reference) (Other :type Actor%20Object%20Reference) (OtherComp :type Primitive%20Component%20Object%20Reference) (bSelfMoved :type Boolean) (HitLocation :type Vector :default "0, 0, 0") (HitNormal :type Vector :default "0, 0, 0") (NormalImpulse :type Vector :default "0, 0, 0") (Hit :type Hit%20Result%20Structure%20%28by%20ref%29))
  (bind _returnvalue (Transformation|GetComponentVelocity MyComp))
  (bind _returnvalue_2 (Physics|GetMass MyComp))
  (bind _returnvalue_3 (Math|Vector|VectorLength _returnvalue))
  (bind _returnvalue_4 (* _returnvalue_3 _returnvalue_2))
  (bind _returnvalue_5 (/ _returnvalue_4 2e+02))
  ;[1 1 1] 소음 이벤트
  (Utilities|FlowControl|Delay 0.5)
  (if (< _returnvalue_5 (Variables|Default|GetMaxNoise))
    (Class|AISenseHearing|ReportNoiseEvent HitLocation _returnvalue_5 0 0.0 "None")
    (else
      (Class|AISenseHearing|ReportNoiseEvent HitLocation (Variables|Default|GetMaxNoise) 0 0.0 "None"))))

(event EventDrop
  ;[1 1 1] PickUp 이벤트
  (Physics|SetSimulatePhysics (Variables|Default|GetStaticMeshComponent) true)
  (Transformation|DetachFromActor "KeepWorld" "KeepWorld" "KeepWorld")
  (Actor|Tick|SetActorTickEnabled false)
  (Effects|Particles|Trails|EndTrails (Variables|Default|GetWaterFall)))

(event EventTick
  (params (DeltaSeconds :type Float%20%28single-precision%29))
  (bind _staticmeshcomponent (Variables|Default|GetStaticMeshComponent))
  (bind _waterfall (Variables|Default|GetWaterFall))
  (bind _waterfall_2 (Variables|Default|GetWaterFall))
  (bind _returnvalue (Transformation|GetWorldTransform _waterfall))
  (bind _returnvalue_2 (Transformation|GetWorldRotation _staticmeshcomponent))
  ;[1 1 1] 물 나오게 하는 코드
  (if (Math|Boolean|ORBoolean (>= (.roll _returnvalue_2) 75.0) (>= (.yaw _returnvalue_2) 75.0) (<= (.roll _returnvalue_2) -75.0) (<= (.yaw _returnvalue_2) -75.0))
    (Effects|Particles|Trails|BeginTrails _waterfall_2 "None" "None" "ETrailWidthMode_FromCentre" 0.0)
    (Utilities|FlowControl|Delay 0.1)
    (Game|SpawnActorfromClass "/Game/LMS/Blueprints/BP_Object/BP_WaterCollision.BP_WaterCollision_C" (Math|Transform|MakeTransform (.location _returnvalue) (.rotation _returnvalue) "0.020000,0.020000,0.020000") "Undefined" 0 0)
    (else
      (Effects|Particles|Trails|EndTrails _waterfall_2))))

(fn ConstructionScript
  (|CallParentFunction))