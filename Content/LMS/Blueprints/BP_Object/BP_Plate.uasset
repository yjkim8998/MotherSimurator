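; BP_Plate is a plate object that can be picked up and dropped.
; Pickup disables physics on the Plate component and attaches the actor's root to the given component, while Drop restores physics and detaches it.
; A gate opened by Pickup and closed by Drop lets Tick move SMPlateDM to the Plate's world location while held.
; The Hit event is empty and the SetDestructibleMesh call is unconnected, so no breaking logic runs.
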(event EventBeginPlay)

(event Collision|EventActorBeginOverlap
  (params (OtherActor :type Actor%20Object%20Reference)))

(event EventTick
  (params (DeltaSeconds :type Float%20%28single-precision%29))
  ;[1 1 1] PickUp 이벤트
  (Utilities|FlowControl|Gate true
    (:Exit
      (Variables|Default|SetPlatePosition (Transformation|GetWorldLocation (Variables|Default|GetPlate)))
      (Transformation|SetWorldLocation (Variables|Default|GetSM_Plate_DM) (Variables|Default|GetPlatePosition) false false))))

(event EventPickup
  (params (AttachTo :type Scene%20Component%20Object%20Reference))
  ;[1 1 1] PickUp 이벤트
  (Physics|SetSimulatePhysics (Variables|Default|GetPlate) false)
  (Transformation|AttachComponentToComponent (VehicleSound|GetRootComponent) AttachTo "None" "KeepWorld" "KeepWorld" "KeepWorld" false)
  (Utilities|FlowControl|Gate true) ; enters at Open
)

(event Collision|EventHit
  (params (MyComp :type Primitive%20Component%20Object%20Reference) (Other :type Actor%20Object%20Reference) (OtherComp :type Primitive%20Component%20Object%20Reference) (bSelfMoved :type Boolean) (HitLocation :type Vector :default "0, 0, 0") (HitNormal :type Vector :default "0, 0, 0") (NormalImpulse :type Vector :default "0, 0, 0") (Hit :type Hit%20Result%20Structure%20%28by%20ref%29)))

(event EventDrop
  ;[1 1 1] PickUp 이벤트
  (Physics|SetSimulatePhysics (Variables|Default|GetPlate) true)
  (Transformation|DetachFromActor "KeepWorld" "KeepWorld" "KeepWorld")
  (Utilities|FlowControl|Gate true) ; enters at Close
)

(fn ConstructionScript)