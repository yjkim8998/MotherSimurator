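; BP_RemoteControl is a remote that can be picked up, dropped and used to switch a flat-screen TV on or off.
; Pickup and Drop toggle physics and attach or detach the actor.
; Interect runs two debug-drawn line traces of different lengths along its negative right vector.
; Each feeds shared logic that, on hitting a BP_FlatTv, toggles the FlatTV reference via TVStat, so one press can toggle twice.
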(event EventInterect
  (bind _remotecontrol (Variables|Default|GetRemoteControl))
  (bind _flattv (Variables|Default|GetFlatTV))
  (bind _returnvalue (Math|Vector|GetRightVector _remotecontrol))
  (bind _returnvalue_2 (Transformation|GetWorldLocation _remotecontrol))
  (bind _returnvalue_3 (+ _returnvalue_2 1e+01))
  (Utilities|FlowControl|Sequence
    (:then_0
      (bind _outhit (Collision|LineTraceByChannel _returnvalue_3 (+ (* (* _returnvalue -1.0) 1e+03) _returnvalue_3) "TraceTypeQuery1" false 0 "ForDuration"))
      (Utilities|Casting|CastToBP_FlatTv (.HitActor (Collision|BreakHitResult _outhit))
        (:then
          (Variables|Default|SetTraceHitFlatTV true :!label _label))
        (:CastFailed
          (Variables|Default|SetTraceHitFlatTV false :!label _label_2))))
    (:then_1
      (bind _outhit_2 (Collision|LineTraceByChannel _returnvalue_3 (+ (* (* _returnvalue -0.5) 1e+03) _returnvalue_3) "TraceTypeQuery1" false 0 "ForDuration"))
      (Utilities|Casting|CastToBP_FlatTv (.HitActor (Collision|BreakHitResult _outhit_2))
        (:then
          (goto _label))
        (:CastFailed
          (goto _label_2)))))
  (if (Variables|Default|GetTraceHitFlatTV)
    (if (Variables|Default|GetTVStat)
      (Default|TurnOffTV _flattv)
      (Variables|Default|SetTVStat false)
      (else
        (Default|TurnonTV _flattv)
        (Variables|Default|SetTVStat true)))))

(event EventPickup
  (params (AttachTo :type Scene%20Component%20Object%20Reference))
  (Physics|SetSimulatePhysics (Variables|Default|GetRemoteControl) false)
  (Transformation|AttachComponentToComponent (VehicleSound|GetRootComponent) AttachTo "None" "KeepWorld" "KeepWorld" "KeepWorld" false))

(event EventDrop
  (Physics|SetSimulatePhysics (Variables|Default|GetRemoteControl) true)
  (Transformation|DetachFromActor "KeepWorld" "KeepWorld" "KeepWorld"))

(fn ConstructionScript)