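; Induction cooktop for a VR cooking interaction, switched on and off when a motion controller overlaps its Hit volume, with the button moving to match.
; Frying pans entering the Trigger volume register it as their Gasrange and clear that on exit.
; While on, a DoOnce-guarded one-second Delay loop calls Fire on overlapping pans.
; Switching off calls CheckCookWithFood on those pans, and the loop resets its guard when it next finds power off.
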(event OnComponentBeginOverlap(Trigger)
  (params (OverlappedComponent :type Primitive%20Component%20Object%20Reference) (OtherActor :type Actor%20Object%20Reference) (OtherComp :type Primitive%20Component%20Object%20Reference) (OtherBodyIndex :type Integer) (bFromSweep :type Boolean) (SweepResult :type Hit%20Result%20Structure%20%28by%20ref%29))
  (bind _asbp_frying_pan (Utilities|Casting|CastToBP_FryingPan OtherActor))
  (Variables|/Game/LMS/Blueprints/Object/BP_FryingPan.BP_FryingPan_C|SetGasrange _asbp_frying_pan self))

(event OnComponentEndOverlap(Trigger)
  (params (OverlappedComponent :type Primitive%20Component%20Object%20Reference) (OtherActor :type Actor%20Object%20Reference) (OtherComp :type Primitive%20Component%20Object%20Reference) (OtherBodyIndex :type Integer))
  (bind _asbp_frying_pan (Utilities|Casting|CastToBP_FryingPan OtherActor))
  (Variables|/Game/LMS/Blueprints/Object/BP_FryingPan.BP_FryingPan_C|SetGasrange _asbp_frying_pan 0))

(event OnComponentBeginOverlap(hit)
  (params (OverlappedComponent :type Primitive%20Component%20Object%20Reference) (OtherActor :type Actor%20Object%20Reference) (OtherComp :type Primitive%20Component%20Object%20Reference) (OtherBodyIndex :type Integer) (bFromSweep :type Boolean) (SweepResult :type Hit%20Result%20Structure%20%28by%20ref%29))
  (bind _button (Variables|Default|GetButton))
  (Utilities|Casting|CastToBP_MotionController OtherActor)
  (if (Variables|Default|GetTurnOnOff)
    (Transformation|AddRelativeLocation _button "0.000000,0.000000,2.000000" false false)
    (Variables|Default|SetTurnOnOff false)
    (for _array_element (Collision|GetOverlappingActors (Variables|Default|GetTrigger) "/Game/LMS/Blueprints/Object/BP_FryingPan.BP_FryingPan_C" :!class /Script/Engine.PrimitiveComponent)
      (bind _asbp_frying_pan (Utilities|Casting|CastToBP_FryingPan _array_element))
      (Default|CheckCookwithFood _asbp_frying_pan))
    (else
      (Transformation|AddRelativeLocation _button "0.000000,0.000000,-2.000000" false false)
      (Variables|Default|SetTurnOnOff true)
      (CallFunction|CookwithFryingfan))))

(event Custom|Cook%20With%20Fryingfan
  (Utilities|FlowControl|DoOnce false :!label _label
    (:Completed
      (Utilities|FlowControl|Delay 1.0 :!label _label_2)
      (if (Variables|Default|GetTurnOnOff)
        (Utilities|FlowControl|Sequence
          (:then_0
            (for _array_element (Collision|GetOverlappingActors (Variables|Default|GetTrigger) "/Game/LMS/Blueprints/Object/BP_FryingPan.BP_FryingPan_C" :!class /Script/Engine.PrimitiveComponent)
              (bind _asbp_frying_pan (Utilities|Casting|CastToBP_FryingPan _array_element))
              (Default|Fire _asbp_frying_pan)))
          (:then_1
            (goto _label_2)))
        (else
          (goto _label Reset))))))

(fn ConstructionScript)