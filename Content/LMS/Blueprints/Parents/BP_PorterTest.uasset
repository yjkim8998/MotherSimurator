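; BP_PorterTest is a physics container prop that can be picked up and dropped, filled with water, then boiled.
; Hits against BP_WaterCollision raise WaterState until full, then reset it, swap the material and enable Tick.
; Tick raises the same counter on a delay until boiled, then swaps to the ready material and stops.
; It passes itself to its water widget, and impacts report AI noise scaled by velocity and mass.
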(event Collision|EventActorBeginOverlap
  (params (OtherActor :type Actor%20Object%20Reference))
  (|CallParentFunction OtherActor) ; 지금 이 노드는 비활성 상태입니다. \n핀을 끌어서 다른 노드를 연결하면 활성화됩니다.
)

(event EventPickup
  (params (AttachTo :type Scene%20Component%20Object%20Reference))
  (Physics|SetSimulatePhysics (Variables|Default|GetStaticMeshComponent) false)
  (Transformation|AttachComponentToComponent (VehicleSound|GetRootComponent) AttachTo "None" "KeepWorld" "KeepWorld" "KeepWorld" false))

(event EventBeginPlay
  (bind _asbpw_water_complete (Utilities|Casting|CastToBPW_Water_Complete (UserInterface|GetUserWidgetObject (Variables|Default|GetWidget))))
  (Variables|/Game/LMS/Blueprints/Widget/BPW_Water_Complete.BPW_Water_Complete_C|SetWater _asbpw_water_complete self))

(event EventDrop
  (Physics|SetSimulatePhysics (Variables|Default|GetStaticMeshComponent) true)
  (Transformation|DetachFromActor "KeepWorld" "KeepWorld" "KeepWorld"))

(event EventTick
  (params (DeltaSeconds :type Float%20%28single-precision%29))
  (Utilities|FlowControl|Delay 0.5)
  (if (< (Variables|Default|GetWater%20State) (Variables|Default|GetMaxBoilWater))
    (Variables|Default|SetWater%20State (+ (Variables|Default|GetWater%20State) (Variables|Default|GetIncreaseWater)))
    (else
      (Actor|Tick|SetActorTickEnabled false)
      (Rendering|Material|SetMaterial (Variables|Default|GetStaticMeshComponent) 0 "/Game/LMS/Materials/Ready_Meterial.Ready_Meterial")
      (Variables|Default|SetisWaterBoil true))))

(event Collision|EventHit
  (params (MyComp :type Primitive%20Component%20Object%20Reference) (Other :type Actor%20Object%20Reference) (OtherComp :type Primitive%20Component%20Object%20Reference) (bSelfMoved :type Boolean) (HitLocation :type Vector :default "0, 0, 0") (HitNormal :type Vector :default "0, 0, 0") (NormalImpulse :type Vector :default "0, 0, 0") (Hit :type Hit%20Result%20Structure%20%28by%20ref%29))
  (CallFunction|WaterHit Other)
  (Utilities|FlowControl|Delay 0.5)
  (Class|AISenseHearing|ReportNoiseEvent HitLocation (/ (* (Math|Vector|VectorLength (Transformation|GetComponentVelocity MyComp)) (Physics|GetMass MyComp)) 1.0) 0 0.0 "None"))

(fn ConstructionScript
  (|CallParentFunction))

(fn WaterHit
  (params (object :type Object%20Object%20Reference))
  (Development|PrintString (Utilities|GetDisplayName object))
  (Utilities|Casting|CastToBP_WaterCollision object
    (:then
      (Development|PrintString "true")
      (if (not (Variables|Default|GetisWaterFull))
        (if (< (Variables|Default|GetWater%20State) (Variables|Default|GetMaxWater))
          (Variables|Default|SetWater%20State (+ (Variables|Default|GetWater%20State) (Variables|Default|GetIncreaseWater)))
          (else
            (Variables|Default|SetisWaterFull true)
            (Variables|Default|SetWater%20State 0.0)
            (Rendering|Material|SetMaterial (Variables|Default|GetStaticMeshComponent) 0 "/Game/LMS/Materials/Waterfull_Material.Waterfull_Material")
            (Actor|Tick|SetActorTickEnabled true)))))
    (:CastFailed
      (Development|PrintString "fail"))))