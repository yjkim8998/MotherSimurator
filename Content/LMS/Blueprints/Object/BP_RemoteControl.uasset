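; BP_RemoteControl is a remote that can be picked up and dropped to switch a BP_FlatTv on and off.
; Pickup and Drop toggle physics, attachment and the WidgetInteraction debug display.
; Interect traces forward from the remote and, on hitting a TV, toggles power using its own TVStat flag.
; The on/off calls go to the FlatTV variable rather than the traced actor.
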(event EventInterect
  (bind _remotecontrol (Variables|Default|GetRemoteControl))
  (bind _flattv (Variables|Default|GetFlatTV))
  (bind _returnvalue (Transformation|GetWorldLocation _remotecontrol))
  (bind _outhit (Collision|LineTraceByChannel _returnvalue (+ (* (Math|Vector|GetForwardVector _remotecontrol) 1e+03) _returnvalue) "TraceTypeQuery1" false 0 "ForDuration"))
  (Utilities|Casting|CastToBP_FlatTv (.HitActor (Collision|BreakHitResult _outhit))
    (:then
      (Variables|Default|SetTraceHitFlatTV true))
    (:CastFailed
      (Variables|Default|SetTraceHitFlatTV false)))
  (if (Variables|Default|GetTraceHitFlatTV)
    (if (Variables|Default|GetTVStat)
      (Default|TurnOffTV _flattv)
      (Variables|Default|SetTVStat false)
      (else
        (Default|TurnonTV _flattv)
        (Variables|Default|SetTVStat true)))))

(event EventPickup
  (params (AttachTo :type Scene%20Component%20Object%20Reference))
  (Physics|SetSimulatePhysics (Variables|Default|GetRemoteControl) false)
  (Transformation|AttachComponentToComponent (VehicleSound|GetRootComponent) AttachTo "None" "KeepWorld" "KeepWorld" "KeepWorld" false)
  (Variables|/Script/UMG.WidgetInteractionComponent|SetbShowDebug (Variables|Default|GetWidgetInteraction) true))

(event EventDrop
  (Physics|SetSimulatePhysics (Variables|Default|GetRemoteControl) true)
  (Transformation|DetachFromActor "KeepWorld" "KeepWorld" "KeepWorld")
  (Variables|/Script/UMG.WidgetInteractionComponent|SetbShowDebug (Variables|Default|GetWidgetInteraction) false))

(fn ConstructionScript)