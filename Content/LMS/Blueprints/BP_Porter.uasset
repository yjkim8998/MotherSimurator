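; BP_Porter is a physics water pot that can be picked up and dropped, fills with water, then boils.
; Overlapping a BP_WaterBottle enables Tick, which uses Delay to throttle the fill; once full, it boils even without the bottle, swapping materials at each stage.
; Four BPW_Water_Complete widgets receive a reference to it on BeginPlay.
; Hits report AI noise scaled by mass times velocity, using MaxNoise for hard impacts.
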(event EventBeginPlay
  ;[1 1 1] Widget 관리
  (bind _asbpw_water_complete (Utilities|Casting|CastToBPW_Water_Complete (UserInterface|GetUserWidgetObject (Variables|Default|GetWidget))))
  (Variables|/Game/LMS/Blueprints/BP_Widget/BPW_Water_Complete.BPW_Water_Complete_C|SetWater _asbpw_water_complete self)
  (bind _asbpw_water_complete_2 (Utilities|Casting|CastToBPW_Water_Complete (UserInterface|GetUserWidgetObject (Variables|Default|GetWidget1))))
  (Variables|/Game/LMS/Blueprints/BP_Widget/BPW_Water_Complete.BPW_Water_Complete_C|SetWater _asbpw_water_complete_2 self)
  (bind _asbpw_water_complete_3 (Utilities|Casting|CastToBPW_Water_Complete (UserInterface|GetUserWidgetObject (Variables|Default|GetWidget3))))
  (Variables|/Game/LMS/Blueprints/BP_Widget/BPW_Water_Complete.BPW_Water_Complete_C|SetWater _asbpw_water_complete_3 self)
  (bind _asbpw_water_complete_4 (Utilities|Casting|CastToBPW_Water_Complete (UserInterface|GetUserWidgetObject (Variables|Default|GetWidget4))))
  (Variables|/Game/LMS/Blueprints/BP_Widget/BPW_Water_Complete.BPW_Water_Complete_C|SetWater _asbpw_water_complete_4 self))

(event Collision|EventActorBeginOverlap
  (params (OtherActor :type Actor%20Object%20Reference))
  ;[1 1 1] Overlap 이벤트
  (if (not (Variables|Default|Getwaterfull))
    (Utilities|Casting|CastToBP_WaterBottle OtherActor)
    (Actor|Tick|SetActorTickEnabled (Variables|Default|Gettrue))))

(event EventPickup
  (params (AttachTo :type Scene%20Component%20Object%20Reference))
  ;[1 1 1] Pickup Drop 이벤트
  (Physics|SetSimulatePhysics (Variables|Default|GetPorter) false)
  (Transformation|AttachComponentToComponent (VehicleSound|GetRootComponent) AttachTo "None" "KeepWorld" "KeepWorld" "KeepWorld" false))

(event Collision|EventHit
  (params (MyComp :type Primitive%20Component%20Object%20Reference) (Other :type Actor%20Object%20Reference) (OtherComp :type Primitive%20Component%20Object%20Reference) (bSelfMoved :type Boolean) (HitLocation :type Vector :default "0, 0, 0") (HitNormal :type Vector :default "0, 0, 0") (NormalImpulse :type Vector :default "0, 0, 0") (Hit :type Hit%20Result%20Structure%20%28by%20ref%29))
  (bind _returnvalue (Transformation|GetComponentVelocity MyComp))
  (bind _returnvalue_2 (Physics|GetMass MyComp))
  (bind _max_noise (Variables|Default|GetMax_Noise))
  (bind _returnvalue_3 (Math|Vector|VectorLength _returnvalue))
  (bind _returnvalue_4 (* _returnvalue_3 _returnvalue_2))
  (bind _returnvalue_5 (/ _returnvalue_4 2e+02))
  ;[1 1 1] 소음 이벤트
  (Utilities|FlowControl|Delay 0.5)
  (if (< _returnvalue_5 1.0)
    (Class|AISenseHearing|ReportNoiseEvent HitLocation _returnvalue_5 0 0.0 "None")
    (Development|PrintString (Utilities|String|ToString(Float) _returnvalue_5))
    (else
      (Class|AISenseHearing|ReportNoiseEvent HitLocation _max_noise 0 0.0 "None")
      (Development|PrintString (Utilities|String|ToString(Float) _max_noise)))))

(event EventDrop
  ;[1 1 1] Pickup Drop 이벤트
  (Physics|SetSimulatePhysics (Variables|Default|GetPorter) true)
  (Transformation|DetachFromActor "KeepWorld" "KeepWorld" "KeepWorld"))

(event Collision|EventActorEndOverlap
  (params (OtherActor :type Actor%20Object%20Reference))
  ;[1 1 1] Overlap 이벤트
  (if (not (Variables|Default|Getwaterfull))
    (Utilities|Casting|CastToBP_WaterBottle OtherActor)
    (Actor|Tick|SetActorTickEnabled (Variables|Default|Getfalse))))

(event EventTick
  (params (DeltaSeconds :type Float%20%28single-precision%29))
  ;[1 1 1] Tick 이벤트
  (if (Variables|Default|Getwaterfull)
    (Utilities|FlowControl|Delay 0.5)
    (if (< (Variables|Default|Getwater_complete) (Variables|Default|Getmax_boilwater))
      (Variables|Default|Setwater_complete (+ (Variables|Default|Getwater_complete) (Variables|Default|Getincrease_float)))
      (else
        (Actor|Tick|SetActorTickEnabled (Variables|Default|Getfalse))
        (Rendering|Material|SetMaterial (Variables|Default|GetPorter) 0 "/Game/LMS/Materials/Ready_Meterial.Ready_Meterial")
        (Variables|Default|Setwaterboilcomplete (Variables|Default|Gettrue))))
    (else
      (Utilities|FlowControl|Delay 0.5)
      (if (< (Variables|Default|Getwater_complete) (Variables|Default|Getmax_water))
        (Variables|Default|Setwater_complete (+ (Variables|Default|Getwater_complete) (Variables|Default|Getincrease_float)))
        (else
          (Variables|Default|Setwaterfull (Variables|Default|Gettrue))
          (Variables|Default|Setwater_complete (Variables|Default|Getinit))
          (Rendering|Material|SetMaterial (Variables|Default|GetPorter) 0 "/Game/LMS/Materials/Waterfull_Material.Waterfull_Material"))))))

(fn ConstructionScript
  (Transformation|SetActorScale3D (Variables|Default|GetMy%20Scale)))