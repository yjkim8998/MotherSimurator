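; Test fish food actor that cooks while it overlaps a frying pan sitting on a gas range.
; BeginPlay sets its perfect-cook level and food volume, and mesh overlap begin and end toggle Actor Tick.
; Tick runs through a one-second Delay, checks the first overlapping BP_FryingPan, then calls Cooking and prints CookedLevel.
; Tick switches itself off when IsCannotCooking is set.
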(event OnComponentBeginOverlap(StaticMesh)
  (params (OverlappedComponent :type Primitive%20Component%20Object%20Reference) (OtherActor :type Actor%20Object%20Reference) (OtherComp :type Primitive%20Component%20Object%20Reference) (OtherBodyIndex :type Integer) (bFromSweep :type Boolean) (SweepResult :type Hit%20Result%20Structure%20%28by%20ref%29))
  (Actor|Tick|SetActorTickEnabled true))

(event OnComponentEndOverlap(StaticMesh)
  (params (OverlappedComponent :type Primitive%20Component%20Object%20Reference) (OtherActor :type Actor%20Object%20Reference) (OtherComp :type Primitive%20Component%20Object%20Reference) (OtherBodyIndex :type Integer))
  (Actor|Tick|SetActorTickEnabled false))

(event EventBeginPlay
  (Variables|Default|SetPerfectelyCookedLevel 2e+01)
  (Variables|Default|SetFoodVolume 5.0))

(event EventTick
  (params (DeltaSeconds :type Float%20%28single-precision%29))
  (if (Variables|Default|GetIsCannotCooking)
    (Actor|Tick|SetActorTickEnabled false)
    (else
      (Utilities|FlowControl|Delay 1.0)
      (bind _asbp_frying_pan (Utilities|Casting|CastToBP_FryingPan (Utilities|Array|Get(acopy) (Collision|GetOverlappingActors "/Game/LMS/Blueprints/Object/BP_FryingPan.BP_FryingPan_C" :!class /Script/Engine.Actor))))
      (if (Variables|/Game/LMS/Blueprints/Object/BP_FryingPan.BP_FryingPan_C|GetIsOnGasrange _asbp_frying_pan)
        (CallFunction|Cooking)
        (Development|PrintString (Utilities|String|ToString(Float) (Variables|Default|GetCookedLevel)))))))

(fn ConstructionScript)