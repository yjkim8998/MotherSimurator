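; BP_Snack_test is a test snack prop actor that can be picked up and dropped.
; Pickup turns off physics, attaches the root to the passed component and snaps the Snack mesh to a fixed relative offset and rotation.
; Calling Pickup again while IsPickup is set swaps the mesh to Snack_test2 instead of reattaching.
; Drop restores physics, detaches the actor keeping world transform and clears the flag.
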(event EventBeginPlay)

(event Collision|EventActorBeginOverlap
  (params (OtherActor :type Actor%20Object%20Reference)))

(event EventTick
  (params (DeltaSeconds :type Float%20%28single-precision%29)))

(event EventPickup
  (params (AttachTo :type Scene%20Component%20Object%20Reference))
  (if (Variables|Default|GetIsPickup)
    (Components|StaticMesh|SetStaticMesh (Variables|Default|GetSnack) "/Game/LMS/snack_test2.snack_test2")
    (else
      (Physics|SetSimulatePhysics (Variables|Default|GetSnack) false)
      (Transformation|AttachComponentToComponent (VehicleSound|GetRootComponent) AttachTo "None" "KeepWorld" "KeepWorld" "KeepWorld" false)
      (Variables|Default|SetIsPickup true)
      (Transformation|SetRelativeLocationAndRotation (Variables|Default|GetSnack) "-5.000000, 0, 0" "0,90.000000, 0" false false))))

(event EventDrop
  (Physics|SetSimulatePhysics (Variables|Default|GetSnack) true)
  (Transformation|DetachFromActor "KeepWorld" "KeepWorld" "KeepWorld")
  (Variables|Default|SetIsPickup false))

(fn ConstructionScript)