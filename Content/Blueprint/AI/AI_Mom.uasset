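; AI controller for the Mom enemy, running BT_Mom and switching Patrol, Look Back, Check Noise and Chase modes with speed and audio changes.
; Sight toggles body and head references per perception update: body triggers Chase instantly, head alone fills a detection meter shown on her eye.
; Hearing escalates modes by loudness and navigation path length, writing the location to the blackboard.
; Footsteps accumulate in a decaying counter that re-emits noise.
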(event Custom|Change%20Mode
  (params (Mode :type BPE_MomMode%20Enum :default "NewEnumerator0"))
  (bind _bgm (Variables|ManagerRef|GetBGM))
  ;[1 1 1] Utility
  (if (not (== (Variables|Default|GetMomMode) Mode))
    (bind _output_get (Variables|Default|SetMomMode Mode))
    (AI|Components|Blackboard|SetValueasEnum (AI|GetBlackboard self) (Utilities|Name|MakeLiteralName "Mom Mode") _output_get)
    (Development|PrintString (Utilities|String|Append "Mom Mode  : " (Utilities|String|EnumtoString _output_get)))
    (switch Utilities|FlowControl|Switch|SwitchonBPE_MomMode _output_get
      (:NewEnumerator0
        (CallFunction|SetCHSpeed false)
        (CallFunction|ClearBBNoiseLocation)
        (Default|Stop _bgm true))
      (:NewEnumerator1
        (CallFunction|RandomSurpriseSound :!label _label))
      (:NewEnumerator2
        (CallFunction|SetCHSpeed true)
        (goto _label))
      (:NewEnumerator3
        (CallFunction|SetCHSpeed true)
        (CallFunction|ClearBBNoiseLocation)
        (Default|Play _bgm "chase")
        (Default|PlaySoundOnce (Variables|Default|GetBPA_SoundController) "detect")))))

(event Custom|Set%20CH%20Speed
  (params (Run :type Boolean))
  ;[1 1 1] Utility
  (Default|SetMoveSpeed (.AsCH%20Mom (Utilities|Casting|CastToCH_Mom (Pawn|GetControlledPawn))) Run))

(event Custom|Run%20Tree
  ;[1 1 1] Utility
  (AI|RunBehaviorTree "/Game/Blueprint/AI/BT_Mom.BT_Mom"))

(event Custom|Random%20Surprise%20Sound
  (bind _bpa_soundcontroller (Variables|Default|GetBPA_SoundController))
  (switch int (Math|Random|RandomInteger 4)
    (:0
      (Default|PlaySoundOnce _bpa_soundcontroller "surprise1"))
    (:1
      (Default|PlaySoundOnce _bpa_soundcontroller "surprise2"))
    (:2
      (Default|PlaySoundOnce _bpa_soundcontroller "surprise3"))
    (:3
      (Default|PlaySoundOnce _bpa_soundcontroller "surprise4"))))

(event EventBeginPlay
  ;[1 1 1] Utility
  (AI|RunBehaviorTree "/Game/Blueprint/AI/BT_Mom.BT_Mom"))

(event OnTargetPerceptionUpdated(AIPerception_Sight)
  (params (Actor :type Actor%20Object%20Reference) (Stimulus :type AI%20Stimulus%20Structure))
  (Variables|Sight|SetDetectedActor Actor)
  (bind _asmotion_controller_pawn (Utilities|Casting|CastToMotionControllerPawn Actor)
    (:then
      (Utilities|IsValid (Variables|Sight|GetPlayerBody)
        (:Is%20Valid
          (CallFunction|Body false)
          (Variables|Sight|SetPlayerBody 0)
          (Utilities|IsValid (Variables|Sight|GetPlayerHead)
            (:Is%20Valid
              (Development|PrintString "쫓다가 머리만 보임 유지"))
            (:Is%20Not%20Valid
              (Development|PrintString "놓침 게이지 1로"))))
        (:Is%20Not%20Valid
          (CallFunction|Body true)
          (Variables|Sight|SetPlayerBody _asmotion_controller_pawn)
          (Development|PrintString "몸발견")
          (Actor|Tick|SetActorTickEnabled true))))
    (:CastFailed
      (bind _asthird_person_character (Utilities|Casting|CastToThirdPersonCharacter Actor)
        (:then
          (Utilities|IsValid (Variables|Sight|GetPlayerBody)
            (:Is%20Valid
              (CallFunction|Body false)
              (Variables|Sight|SetPlayerBody 0)
              (Utilities|IsValid (Variables|Sight|GetPlayerHead)
                (:Is%20Valid
                  (Development|PrintString "쫓다가 머리만 보임 유지"))
                (:Is%20Not%20Valid
                  (Development|PrintString "놓침 게이지 1로"))))
            (:Is%20Not%20Valid
              (CallFunction|Body true)
              (Variables|Sight|SetPlayerBody _asthird_person_character)
              (Development|PrintString "몸발견")
              (Actor|Tick|SetActorTickEnabled true))))
        (:CastFailed
          (bind _asbp_head (Utilities|Casting|CastToBP_Head Actor))
          (Utilities|IsValid (Variables|Sight|GetPlayerHead)
            (:Is%20Valid
              (CallFunction|Head false)
              (Variables|Sight|SetPlayerHead 0)
              (Utilities|IsValid (Variables|Sight|GetPlayerBody)
                (:Is%20Valid
                  (Development|PrintString "머리 놓치고 몸 발견상태"))
                (:Is%20Not%20Valid
                  (Development|PrintString "머리만 인식하다 놓침"))))
            (:Is%20Not%20Valid
              (CallFunction|Head true)
              (Variables|Sight|SetPlayerHead _asbp_head)
              (Utilities|IsValid (Variables|Sight|GetPlayerBody)
                (:Is%20Valid
                  (Development|PrintString "몸 발견상태에서 머리추가 발견"))
                (:Is%20Not%20Valid
                  (Development|PrintString "머리만 발견")
                  (Actor|Tick|SetActorTickEnabled true))))))))))

(event Custom|Set%20Eye%20Percent
  (bind _asch_mom (Utilities|Casting|CastToCH_Mom (Pawn|GetControlledPawn)))
  (Default|SetEyePercent _asch_mom (Variables|Sight|GetDetectMeter)))

(event Custom|body
  (params (NewParam :type Boolean))
  (Default|SetBody (.AsCH%20Mom (Utilities|Casting|CastToCH_Mom (Pawn|GetControlledPawn))) NewParam))

(event Custom|set%20text2
  (params (NewParam :type String))
  ;[1 1 1] Utility
  (Default|SetMomHeadText2 (.AsCH%20Mom (Utilities|Casting|CastToCH_Mom (Pawn|GetControlledPawn))) NewParam))

(event Custom|head
  (params (NewParam :type Boolean))
  (Default|SetHead (.AsCH%20Mom (Utilities|Casting|CastToCH_Mom (Pawn|GetControlledPawn))) NewParam))

(event EventTick
  (params (DeltaSeconds :type Float%20%28single-precision%29))
  (Utilities|FlowControl|Sequence
    (:then_0
      (Utilities|IsValid (Variables|Sight|GetPlayerBody)
        (:Is%20Valid
          (Variables|Sight|SetDetectMeter 1.0)
          (CallFunction|ChangeMode "NewEnumerator3"))
        (:Is%20Not%20Valid
          (Utilities|IsValid (Variables|Sight|GetPlayerHead)
            (:Is%20Valid
              (if (< (Variables|Sight|GetDetectMeter) 1.0)
                (Variables|Sight|SetDetectMeter (+ (Variables|Sight|GetDetectMeter) 0.025))
                (else
                  (CallFunction|ChangeMode "NewEnumerator3"))))
            (:Is%20Not%20Valid
              (if (> (Variables|Sight|GetDetectMeter) 0.0)
                (Variables|Sight|SetDetectMeter (- (Variables|Sight|GetDetectMeter) 0.025))))))))
    (:then_1
      (CallFunction|SetEyePercent))))

(event OnTargetPerceptionUpdated(AIPerception_Nosie)
  (params (Actor :type Actor%20Object%20Reference) (Stimulus :type AI%20Stimulus%20Structure))
  (if (Utilities|Name|NotEqual(Name) (.tag Stimulus) "Step")
    (CallFunction|CompareNoise (.strength Stimulus) (.stimuluslocation Stimulus))
    (switch Utilities|FlowControl|Switch|SwitchonBPE_MomMode (Variables|Default|GetMomMode)
      (:NewEnumerator0
        (if (>= (Variables|Noise|GetCurrentNoise) 0.2)
          (if (>= (Variables|Noise|GetCurrentNoise) 0.8)
            (bind _in_range (CallFunction|GetBetweenDistance (.stimuluslocation Stimulus) 3e+03))
            (if _in_range
              (CallFunction|ChangeMode "NewEnumerator2"))
            (else
              (bind _in_range_2 (CallFunction|GetBetweenDistance (.stimuluslocation Stimulus) 1.5e+03))
              (if _in_range_2
                (CallFunction|ChangeMode "NewEnumerator1"))))))
      (:NewEnumerator1
        (if (>= (Variables|Noise|GetCurrentNoise) 0.2)
          (CallFunction|ChangeMode "NewEnumerator2"))))
    (else
      (CallFunction|GetStep (.stimuluslocation Stimulus)))))

(event Custom|Compare%20Noise
  (params (Noise%20Strength :type Float%20%28single-precision%29) (Location :type Vector))
  ;[1 1 1] Utility
  (if (>= Noise%20Strength (Variables|Noise|GetCurrentNoise))
    (Variables|Noise|SetCurrentNoise Noise%20Strength)
    (CallFunction|SetBBNoiseLocation Location)))

(event Custom|Clear%20Noise
  ;[1 1 1] Utility
  (Variables|Noise|SetCurrentNoise 0.0)
  (AI|Components|Blackboard|ClearValue (AI|GetBlackboard self) (Utilities|Name|MakeLiteralName "Noise Location")))

(event Custom|Clear%20BB%20NoiseLocation
  ;[1 1 1] Utility
  (AI|Components|Blackboard|ClearValue (AI|GetBlackboard self) (Utilities|Name|MakeLiteralName "Noise Location"))
  (Variables|Noise|SetCurrentNoise 0.0))

(event Custom|Get%20Step
  (params (Location :type Vector))
  ;[1 1 1] Utility
  (Variables|Noise|SetStepNoise (+ (Variables|Noise|GetStepNoise) 0.5))
  (Utilities|FlowControl|DoOnce false :!label _label
    (:Completed
      (if (> (Variables|Noise|GetStepNoise) 0.0) :!label _label_2
        (Variables|Noise|SetStepNoise (- (Variables|Noise|GetStepNoise) 0.05))
        (if (>= (Variables|Noise|GetStepNoise) 1.0)
          (Class|Actor|MakeNoise 0.5 0 Location 0.0 "None")
          (Variables|Noise|SetStepNoise 0.0)
          (goto _label_2)
          (else
            (Utilities|FlowControl|Delay 0.1)
            (goto _label_2)))
        (else
          (goto _label Reset))))))

(event Custom|Set%20BB%20NoiseLocation
  (params (Noise%20Location :type Vector))
  ;[1 1 1] Utility
  (AI|Components|Blackboard|SetValueasVector (AI|GetBlackboard self) (Utilities|Name|MakeLiteralName "Noise Location") Noise%20Location))

(fn ConstructionScript)

(fn GetBetweenDistance
  (params (Target%20Location :type Vector) (Distance :type Float%20%28single-precision%29))
  (return (<= (.PathLength (Class|NavigationSystemV1|GetPathLength (Transformation|GetActorLocation (Pawn|GetControlledPawn)) Target%20Location 0 0)) Distance)))