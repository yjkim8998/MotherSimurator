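; Test AI controller, apparently for a "Mom" character, that runs the BT_Test behavior tree on BeginPlay.
; Any AI Perception target update writes the stimulus location to the "Noise Location" blackboard key and switches to one fixed Mom Mode, without filtering the stimulus.
; Helper events set or clear the noise location and change the mode, mirroring it to the blackboard with a debug print.
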(event OnTargetPerceptionUpdated(AIPerception)
  (params (Actor :type Actor%20Object%20Reference) (Stimulus :type AI%20Stimulus%20Structure))
  (CallFunction|SetBBNoiseLocation (.stimuluslocation Stimulus))
  (CallFunction|ChangeMode "NewEnumerator2"))

(event Custom|Change%20Mode
  (params (Mode :type BPE_MomMode%20Enum :default "NewEnumerator0"))
  (bind _output_get (Variables|Default|SetMomMode Mode))
  (AI|Components|Blackboard|SetValueasEnum (AI|GetBlackboard self) (Utilities|Name|MakeLiteralName "Mom Mode") _output_get)
  (Development|PrintString (Utilities|String|Append "Mom Mode  : " (Utilities|String|EnumtoString _output_get))))

(event Custom|Clear%20Noise
  (AI|Components|Blackboard|ClearValue (AI|GetBlackboard self) (Utilities|Name|MakeLiteralName "Noise Location")))

(event Custom|Set%20BB%20NoiseLocation
  (params (Noise%20Location :type Vector))
  (AI|Components|Blackboard|SetValueasVector (AI|GetBlackboard self) (Utilities|Name|MakeLiteralName "Noise Location") Noise%20Location))

(event EventBeginPlay
  (AI|RunBehaviorTree "/Game/Blueprint/AI/BT_Test.BT_Test"))

(fn ConstructionScript)