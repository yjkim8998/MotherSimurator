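; BP_ItemManager is an object-pool manager that keeps food items stocked in the game.
; BeginPlay pre-spawns hidden, non-colliding BP_TestFood actors that reference the manager, then activates an initial batch at RoomM spawn points.
; SetActorActive toggles visibility, physics and collision; returned food re-enters the pool, and FoodSupply refills toward the maximum once the active count reaches the low threshold.
; Unique item spawn and return are unfinished stubs.
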(event Custom|Spawn%20Normal%20Food
  (params (Num :type Integer))
  (bind _normalitempool (Variables|Default|GetNormalItemPool))
  (bind _output (Utilities|Array|Get(acopy) _normalitempool))
  ;[1 1 1] Normal Food
  (if (>= (Utilities|Array|Length (Variables|Default|GetNormalItemPool)) Num)
    (for _index (range 1 Num)
      (CallFunction|SetActorActive _output true)
      (bind _spawn_location (Default|GetSpawnVector (Variables|ManagerRef|GetRoomM)))
      (Transformation|Teleport _output _spawn_location "0, 0, 0")
      (Utilities|Array|RemoveIndex (Variables|Default|GetNormalItemPool))
      (Math|Integer|IncrementInt (Variables|Default|GetNormalFoodCount)))))

(event Custom|Spawn%20Unique%20Item
  (params (Unique%20Item :type Actor%20Object%20Reference))
  (Default|GetSpawnVector (Variables|ManagerRef|GetRoomM)))

(event Custom|Set%20Actor%20Active
  (params (Target%20Actor :type BP%20Base%20Food%20Object%20Reference) (Active :type Boolean))
  (bind _staticmesh (Variables|/Game/Blueprint/Base/BP_BaseFood.BP_BaseFood_C|GetStaticMesh Target%20Actor))
  (Development|SetHiddeninGame (Variables|/Script/Engine.Actor|GetRootComponent Target%20Actor) (not Active) false)
  (Physics|SetSimulatePhysics _staticmesh Active)
  (if Active
    (Collision|SetCollisionEnabled _staticmesh "QueryAndPhysics")
    (else
      (Collision|SetCollisionEnabled _staticmesh "NoCollision"))))

(event Custom|Reeturn%20To%20Nomal%20Pool
  (params (Target%20Actor :type BP%20Base%20Food%20Object%20Reference))
  ;[1 1 1] Normal Food
  (Utilities|Array|Add (Variables|Default|GetNormalItemPool) Target%20Actor)
  (CallFunction|SetActorActive Target%20Actor false)
  (Math|Integer|DecrementInt (Variables|Default|GetNormalFoodCount)
    (:%20%20
      (CallFunction|FoodSupply)
      (Development|PrintString "Hello" true true "(R=1.000000,G=0.005868,B=0.000000,A=1.000000)"))))

(event Custom|Food%20Supply
  ;[1 1 1] Normal Food
  (if (<= (Variables|Default|GetNormalFoodCount) (Variables|Default|GetLessNormalFoodCount))
    (CallFunction|SpawnNormalFood (- (Variables|Default|GetMaxNormalFoodCount) (Variables|Default|GetNormalFoodCount)))
    (Development|PrintString "음식 소환" true true "(R=0.062202,G=0.000000,B=1.000000,A=1.000000)")))

(event Custom|Return%20To%20UniquePool
  (params (Target%20Actor :type Actor%20Object%20Reference)))

(event EventBeginPlay
  (Utilities|FlowControl|Sequence
    (:then_0
      (for _index (range 1 30)
        (bind _returnvalue (Game|SpawnActorfromClass "/Game/Blueprint/Obj/Food/BP_TestFood.BP_TestFood_C" (Math|Transform|MakeTransform "0, 0, 0" "0, 0, 0" "0.300000,0.300000,0.300000") "AlwaysSpawn" 0 0))
        (Utilities|Array|Add (Variables|Default|GetNormalItemPool) _returnvalue)
        (Variables|/Game/Blueprint/Base/BP_BaseFood.BP_BaseFood_C|SetItemM _returnvalue self)
        (CallFunction|SetActorActive _returnvalue false)))
    (:then_1
      (CallFunction|SpawnNormalFood 10))))

(fn ConstructionScript)