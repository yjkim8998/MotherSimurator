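; BP_BGM is a background music manager that plays, stops, pauses and resumes one 2D track at a time.
; Play looks up the requested track in the DicBGM map, destroys any playing or fading audio component and starts a newly created 2D sound.
; Stop either destroys the track immediately or moves it to a separate fading slot for a two-second linear fade-out before destroying it.
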(event Custom|Play
  (params (bgm :type Name))
  (bind _fadingbgm (Variables|Default|GetFadingBgm))
  (Utilities|IsValid _fadingbgm
    (:Is%20Valid
      (Components|DestroyComponent _fadingbgm))
    (:Is%20Not%20Valid
      _))
  (Utilities|IsValid (Variables|Default|GetPlayingBgm)
    (:Is%20Valid
      (Components|DestroyComponent (Variables|Default|GetPlayingBgm)))
    (:Is%20Not%20Valid
      _))
  (bind _returnvalue (Audio|CreateSound2D (.Value (Utilities|Map|Find (Variables|Default|GetDic_BGM) bgm)) 1.0 1.0 0.0 0))
  (bind _output_get (Variables|Default|SetPlayingBgm _returnvalue))
  (Audio|Components|Audio|Play _output_get 0.0))

(event Custom|Stop
  (params (Fade :type Boolean))
  (Utilities|IsValid (Variables|Default|GetFadingBgm)
    (:Is%20Valid
      (Components|DestroyComponent (Variables|Default|GetFadingBgm)))
    (:Is%20Not%20Valid
      _))
  (Utilities|IsValid (Variables|Default|GetPlayingBgm)
    (:Is%20Valid
      (if Fade
        (bind _output_get (Variables|Default|SetFadingBgm (Variables|Default|GetPlayingBgm)))
        (Variables|Default|SetPlayingBgm 0)
        (Audio|Components|Audio|FadeOut _output_get 2.0 0.0 "Linear" :!class /Script/Engine.AudioComponent)
        (Utilities|FlowControl|Delay 2.0)
        (Utilities|IsValid (Variables|Default|GetFadingBgm)
          (:Is%20Valid
            (Components|DestroyComponent (Variables|Default|GetFadingBgm))))
        (else
          (Components|DestroyComponent (Variables|Default|GetPlayingBgm)))))))

(event Custom|Pause
  (bind _playingbgm (Variables|Default|GetPlayingBgm))
  (Utilities|IsValid _playingbgm
    (:Is%20Valid
      (Class|AudioComponent|SetPaused _playingbgm true))))

(event Custom|Replay
  (bind _playingbgm (Variables|Default|GetPlayingBgm))
  (Utilities|IsValid _playingbgm
    (:Is%20Valid
      (Class|AudioComponent|SetPaused _playingbgm false))))

(fn ConstructionScript)