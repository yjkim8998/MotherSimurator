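; BP_EventManager is a manager that starts and ends gameplay events drawn from a pool of event objects.
; On BeginPlay it shuffles the pool and hides each event's root component.
; SpawnEvent moves the front event into a running map keyed by an incrementing counter, begins it with index 0 and unhides its root.
; EndEvent ends the event at the given key and returns it to the back of the pool without re-hiding it.
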(event Custom|Spawn%20Event
  (bind _eventpool (Variables|Default|GetEventPool))
  (bind _output (Utilities|Array|Get(acopy) _eventpool))
  (Utilities|Map|Add (Variables|Default|GetRunningEventPool) (Variables|Default|GetEventCount) _output)
  (Default|BeginEvent _output)
  (Development|SetHiddeninGame (Variables|/Game/Blueprint/Event/BP_Event.BP_Event_C|GetDefaultSceneRoot _output) false false)
  (Utilities|Array|RemoveIndex (Variables|Default|GetEventPool))
  (Math|Integer|IncrementInt (Variables|Default|GetEventCount)))

(event Custom|End%20Event
  (params (EventIndex :type Integer))
  (bind _runningeventpool (Variables|Default|GetRunningEventPool))
  (bind _value (Utilities|Map|Find _runningeventpool EventIndex))
  (Default|EndEvent _value)
  (Utilities|Array|Add (Variables|Default|GetEventPool) _value)
  (Utilities|Map|Remove (Variables|Default|GetRunningEventPool) EventIndex))

(event EventBeginPlay
  (Utilities|Array|Shuffle (Variables|Default|GetEventPool))
  (for _array_element (Variables|Default|GetEventPool)
    (Development|SetHiddeninGame (Variables|/Game/Blueprint/Event/BP_Event.BP_Event_C|GetDefaultSceneRoot _array_element) true false)))

(fn ConstructionScript)