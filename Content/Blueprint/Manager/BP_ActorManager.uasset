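; BP_ActorManager is an actor pool for one class, with physics handling for BP_BaseFood actors.
; InitPool pre-spawns hidden, non-colliding copies attached to the manager, disabling physics on food meshes.
; Both getters move the first pooled actor to a location and re-enable it, one also returning it; neither grows an empty pool.
; Returned actors of the pooled class are reattached and hidden with collision left on, while others are destroyed.
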(event Custom|Init%20Pool
  (params (Target%20Actor :type Actor%20Class%20Reference) (Count :type Integer))
  (Variables|Default|SetTargetActorClass Target%20Actor)
  (for _index (range 1 Count)
    (bind _returnvalue (Game|SpawnActorfromClass (Variables|Default|GetTargetActorClass) (Math|Transform|MakeTransform "0, 0, 0" "0, 0, 0" "0.100000,0.100000,0.100000") "AlwaysSpawn" 0 0))
    (Utilities|Array|Add (Variables|Default|GetPool) _returnvalue)
    (Rendering|SetActorHiddenInGame _returnvalue true)
    (Collision|SetActorEnableCollision _returnvalue false)
    (Transformation|AttachActorToActor _returnvalue self "None" "KeepRelative" "KeepRelative" "KeepRelative" true)
    (bind _asbp_base_food (Utilities|Casting|CastToBP_BaseFood _returnvalue))
    (Physics|SetSimulatePhysics (Variables|/Game/Blueprint/Base/BP_BaseFood.BP_BaseFood_C|GetStaticMesh _asbp_base_food) false)))

(event Custom|Get%20Actor%20From%20Pool
  (params (Location :type Vector))
  (bind _pool (Variables|Default|GetPool))
  (bind _output (Utilities|Array|Get(acopy) _pool))
  (if (> (Utilities|Array|Length _pool) 0)
    (Transformation|SetActorLocationAndRotation _output Location "0, 0, 0" false true)
    (Rendering|SetActorHiddenInGame _output false)
    (Collision|SetActorEnableCollision _output true)
    (bind _asbp_base_food (Utilities|Casting|CastToBP_BaseFood _output)
      (:then
        (Physics|SetSimulatePhysics (Variables|/Game/Blueprint/Base/BP_BaseFood.BP_BaseFood_C|GetStaticMesh _asbp_base_food) true))
      (:CastFailed
        _))
    (Utilities|Array|RemoveIndex (Variables|Default|GetPool))))

(event Custom|Return%20Actor%20To%20Pool
  (params (Target%20Actor :type Actor%20Object%20Reference))
  (if (== (Variables|Default|GetTargetActorClass) (Utilities|GetClass Target%20Actor))
    (Utilities|Array|Add (Variables|Default|GetPool) Target%20Actor)
    (Transformation|AttachActorToActor Target%20Actor self "None" "KeepRelative" "KeepRelative" "KeepRelative" true)
    (Rendering|SetActorHiddenInGame Target%20Actor true)
    (Collision|SetActorEnableCollision Target%20Actor true)
    (bind _asbp_base_food (Utilities|Casting|CastToBP_BaseFood Target%20Actor))
    (Physics|SetSimulatePhysics (Variables|/Game/Blueprint/Base/BP_BaseFood.BP_BaseFood_C|GetStaticMesh _asbp_base_food) false)
    (else
      (Actor|DestroyActor Target%20Actor))))

(fn ConstructionScript)

(fn GetActorfromActorPoolReturn
  (params (Location :type Vector))
  (bind _pool (Variables|Default|GetPool))
  (if (> (Utilities|Array|Length _pool) 0)
    (bind _output_get (LocalVariables|SetTarget%20Actor (Utilities|Array|Get(acopy) _pool)))
    (Utilities|Array|RemoveIndex (Variables|Default|GetPool))
    (Transformation|SetActorLocationAndRotation _output_get Location "0, 0, 0" false true)
    (Rendering|SetActorHiddenInGame (LocalVariables|GetTarget%20Actor) false)
    (Collision|SetActorEnableCollision (LocalVariables|GetTarget%20Actor) true)
    (bind _asbp_base_food (Utilities|Casting|CastToBP_BaseFood (LocalVariables|GetTarget%20Actor))
      (:then
        (Physics|SetSimulatePhysics (Variables|/Game/Blueprint/Base/BP_BaseFood.BP_BaseFood_C|GetStaticMesh _asbp_base_food) true))
      (:CastFailed
        _))
    (return (LocalVariables|GetTarget%20Actor))))