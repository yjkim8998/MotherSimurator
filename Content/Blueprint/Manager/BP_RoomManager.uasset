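; Room manager that builds a randomized 4x4 room layout and serves spawn and patrol points.
; InitRoomM shuffles room pools by entrance count, swaps in a kitchen, spaces and rotates rooms, processes door walls and destroys unused rooms.
; InitTP gathers room target points into a non-repeating spawn pool and a score map, intended to favor the kitchen.
; Player sightings raise point scores, empty patrols lower them, and GetNearestPoint searches room, then point.
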(event Custom|Init%20RoomM
  (Utilities|Array|Shuffle (Variables|RoomRef|Get2entrances))
  (Utilities|Array|Shuffle (Variables|RoomRef|Get3entrances))
  (Utilities|Array|Shuffle (Variables|RoomRef|Get4entrances))
  (CallFunction|Clear2DArray)
  (CallFunction|1Make2DArray)
  (CallFunction|2ChangeOnetoKitchen)
  (CallFunction|3RoomSpacing)
  (CallFunction|4FixRoomRoation)
  (CallFunction|5Destroy30%Door)
  (CallFunction|DestroyUnselectedRoom))

(event Custom|Add%202D%20Array%203
  (params (Target%20Item%20Array :type Array%20of%20BP%20Base%20Room%20Object%20References) (Item%20Index :type Integer))
  ;[1 1 1] 선택된 배열에 추가
  (Utilities|Array|Add (Variables|SelRoomRef|Get3) (Utilities|Array|Get(acopy) Target%20Item%20Array Item%20Index)))

(event Custom|Set%20Room%20Location
  (params (Taraget%20Array :type Array%20of%20BP%20Base%20Room%20Object%20References) (X :type Float%20%28single-precision%29))
  ;[1 1 1] 방 X 위치 설정
  (bind _output_get (Variables|RoomSpacing|SetCurrentSpacingX (- (- 0.0 (Variables|RoomSpacing|GetRoomSpacing)) (* (Variables|RoomSpacing|GetRoomSpacing) 0.5))))
  (for _array_element Taraget%20Array
    (Transformation|SetRelativeLocation (Variables|/Script/Engine.Actor|GetRootComponent _array_element) (Math|Vector|MakeVector X _output_get 0.0) false false)
    (Variables|RoomSpacing|SetCurrentSpacingX (+ (Variables|RoomSpacing|GetCurrentSpacingX) (Variables|RoomSpacing|GetRoomSpacing)))))

(event Custom|Set%202%20Rotation
  (params (Index :type Integer) (Rotation%20Z :type Float%20%28single-precision%29))
  ;[1 1 1] 선택된 배열 회전 설정
  (Transformation|SetRelativeRotation (Variables|/Game/Blueprint/Base/BP_BaseRoom.BP_BaseRoom_C|GetDefaultSceneRoot (Utilities|Array|Get(acopy) (Variables|SelRoomRef|Get2) Index)) (Math|Rotator|MakeRotator 0.0 0.0 Rotation%20Z) false false))

(event Custom|Init%20TP
  (bind _indexplus (Variables|Default|GetIndexPlus))
  (for _array_element (Variables|SelRoomRef|Get0)
    (Utilities|Array|Add (Variables|SelRoomRef|GetSelRoom) _array_element))
  (for _array_element_2 (Variables|SelRoomRef|Get1)
    (Utilities|Array|Add (Variables|SelRoomRef|GetSelRoom) _array_element_2))
  (for _array_element_3 (Variables|SelRoomRef|Get2)
    (Utilities|Array|Add (Variables|SelRoomRef|GetSelRoom) _array_element_3))
  (for _array_element_4 (Variables|SelRoomRef|Get3)
    (Utilities|Array|Add (Variables|SelRoomRef|GetSelRoom) _array_element_4))
  (for _array_element_5 (Variables|SelRoomRef|GetSelRoom)
    (Variables|/Game/Blueprint/Base/BP_BaseRoom.BP_BaseRoom_C|SetRoomIndex _array_element_5 _indexplus)
    (Math|Integer|IncrementInt _indexplus
      (:%20%20
        (Transformation|AttachActorToActor _array_element_5 self "None" "KeepRelative" "KeepRelative" "KeepRelative" true)
        (bind _spawnpoint (Default|GetSpawnTP _array_element_5))
        (CallFunction|AddSpawnTP _spawnpoint)
        (CallFunction|AddLocationTP _array_element_5)))))

(event Custom|Set%200%20Rotation
  (params (Index :type Integer) (Rotation%20Z :type Float%20%28single-precision%29))
  ;[1 1 1] 선택된 배열 회전 설정
  (Transformation|SetRelativeRotation (Variables|/Game/Blueprint/Base/BP_BaseRoom.BP_BaseRoom_C|GetDefaultSceneRoot (Utilities|Array|Get(acopy) (Variables|SelRoomRef|Get0) Index)) (Math|Rotator|MakeRotator 0.0 0.0 Rotation%20Z) false false))

(event Custom|Set%201%20Rotation
  (params (Index :type Integer) (Rotation%20Z :type Float%20%28single-precision%29))
  ;[1 1 1] 선택된 배열 회전 설정
  (Transformation|SetRelativeRotation (Variables|/Game/Blueprint/Base/BP_BaseRoom.BP_BaseRoom_C|GetDefaultSceneRoot (Utilities|Array|Get(acopy) (Variables|SelRoomRef|Get1) Index)) (Math|Rotator|MakeRotator 0.0 0.0 Rotation%20Z) false false))

(event Custom|1%20Make%202D%20Array
  ;[1 1 1] 이차원 배열 설정
  (CallFunction|Add2DArray0 (Variables|RoomRef|Get2entrances))
  (CallFunction|Add2DArray0 (Variables|RoomRef|Get3entrances))
  (CallFunction|Add2DArray0 (Variables|RoomRef|Get3entrances) 1)
  (CallFunction|Add2DArray0 (Variables|RoomRef|Get2entrances) 1)
  (CallFunction|Add2DArray1 (Variables|RoomRef|Get3entrances) 2)
  (CallFunction|Add2DArray1 (Variables|RoomRef|Get4entrances))
  (CallFunction|Add2DArray1 (Variables|RoomRef|Get4entrances) 1)
  (CallFunction|Add2DArray1 (Variables|RoomRef|Get3entrances) 3)
  (CallFunction|Add2DArray2 (Variables|RoomRef|Get3entrances) 4)
  (CallFunction|Add2DArray2 (Variables|RoomRef|Get4entrances) 2)
  (CallFunction|Add2DArray2 (Variables|RoomRef|Get4entrances) 3)
  (CallFunction|Add2DArray2 (Variables|RoomRef|Get3entrances) 5)
  (CallFunction|Add2DArray3 (Variables|RoomRef|Get2entrances) 2)
  (CallFunction|Add2DArray3 (Variables|RoomRef|Get3entrances) 6)
  (CallFunction|Add2DArray3 (Variables|RoomRef|Get3entrances) 7)
  (CallFunction|Add2DArray3 (Variables|RoomRef|Get2entrances) 3))

(event Custom|Add%20Location%20TP
  (params (RoomLocationTP :type BP%20Base%20Room%20Object%20Reference))
  (bind _dic_lpscore (Variables|Default|GetDic_LPScore))
  (bind _locationpoint (Default|GetLocationTP RoomLocationTP))
  (if (== (Variables|/Game/Blueprint/Base/BP_BaseRoom.BP_BaseRoom_C|GetRoomIndex RoomLocationTP) (Variables|Default|GetSelKitchen))
    (for _array_element _locationpoint
      (Utilities|Map|Add _dic_lpscore _array_element 15))
    (else
      (for _array_element_2 _locationpoint
        (Utilities|Map|Add _dic_lpscore _array_element_2 5)))))

(event Custom|Spawn%20Wall
  (params (X :type Float%20%28single-precision%29) (Y :type Float%20%28single-precision%29) (width :type Boolean))
  (bind _returnvalue (Game|SpawnActorfromClass "/Game/Blueprint/Obj/Room/Base/BP_DoorWall.BP_DoorWall_C" (Math|Transform|MakeTransform "0, 0, 0" "0, 0, 0" "1,1,1") "Undefined" 0 0))
  (Transformation|AttachComponentToComponent (Variables|/Script/Engine.Actor|GetRootComponent _returnvalue) (Variables|Default|GetDefaultSceneRoot) "None" "KeepRelative" "KeepRelative" "KeepRelative" true)
  (Transformation|SetRelativeLocation (Variables|/Script/Engine.Actor|GetRootComponent _returnvalue) (Math|Vector|MakeVector X Y 5e+01) false false)
  (if width
    (Transformation|SetRelativeRotation (Variables|/Script/Engine.Actor|GetRootComponent _returnvalue) "0, 0, 0" false false)
    (else
      (Transformation|SetRelativeRotation (Variables|/Script/Engine.Actor|GetRootComponent _returnvalue) "0.0,90.000000,0.0" false false))))

(event Custom|Add%20SpawnTP
  (params (RoomSpawnTP :type Array%20of%20BPT%20Spawn%20Point%20Object%20References))
  (for _array_element RoomSpawnTP
    (Utilities|Array|Add (Variables|Default|GetSpawnTP) _array_element)))

(event Custom|Reload%20UniqueTP
  (bind _output_get (Variables|Default|SetSpawnTPConsumable (Variables|Default|GetSpawnTP)))
  (Utilities|Array|Shuffle _output_get))

(event Custom|Clear%202D%20Array
  (Utilities|Array|Clear (Variables|SelRoomRef|Get0))
  (Utilities|Array|Clear (Variables|SelRoomRef|Get1))
  (Utilities|Array|Clear (Variables|SelRoomRef|Get2))
  (Utilities|Array|Clear (Variables|SelRoomRef|Get3)))

(event Custom|2%20Change%20One%20To%20Kitchen
  (bind _returnvalue (Math|Random|RandomInteger 4))
  ;[1 1 1] 주방 교체
  (bind _output_get (Variables|Default|SetSelKitchen (Math|Random|RandomInteger 3)))
  (switch int _output_get
    (:0
      (CallFunction|InsertKitchento2 _returnvalue (Utilities|Array|Get(acopy) (Variables|RoomRef|Getkitchen) _output_get)))
    (:1
      (CallFunction|InsertKitchento3 (Math|Random|RandomInteger 8) (Utilities|Array|Get(acopy) (Variables|RoomRef|Getkitchen) _output_get)))
    (:2
      (CallFunction|InsertKitchento4 _returnvalue (Utilities|Array|Get(acopy) (Variables|RoomRef|Getkitchen) _output_get)))))

(event Custom|3%20Room%20Spacing
  (bind _roomspacing (Variables|RoomSpacing|GetRoomSpacing))
  ;[1 1 1] 방 Y 위치 설정 하고 X호출
  (bind _output_get (Variables|RoomSpacing|SetCurrentSpacingY (+ _roomspacing (/ _roomspacing 2.0))))
  (CallFunction|SetRoomLocation (Variables|SelRoomRef|Get0) _output_get)
  (bind _output_get_2 (Variables|RoomSpacing|SetCurrentSpacingY (- (Variables|RoomSpacing|GetCurrentSpacingY) (Variables|RoomSpacing|GetRoomSpacing))))
  (CallFunction|SetRoomLocation (Variables|SelRoomRef|Get1) _output_get_2)
  (bind _output_get_3 (Variables|RoomSpacing|SetCurrentSpacingY (- (Variables|RoomSpacing|GetCurrentSpacingY) (Variables|RoomSpacing|GetRoomSpacing))))
  (CallFunction|SetRoomLocation (Variables|SelRoomRef|Get2) _output_get_3)
  (bind _output_get_4 (Variables|RoomSpacing|SetCurrentSpacingY (- (Variables|RoomSpacing|GetCurrentSpacingY) (Variables|RoomSpacing|GetRoomSpacing))))
  (CallFunction|SetRoomLocation (Variables|SelRoomRef|Get3) _output_get_4))

(event Custom|4%20Fix%20Room%20Roation
  (bind _returnvalue (Math|Random|RandomInteger 4))
  (bind _returnvalue_2 (* _returnvalue 9e+01))
  ;[1 1 1] 회전
  (CallFunction|Set0Rotation 0 0.0)
  (CallFunction|Set0Rotation 1 0.0)
  (CallFunction|Set0Rotation 2 0.0)
  (CallFunction|Set0Rotation 3 9e+01)
  (CallFunction|Set1Rotation 0 -9e+01)
  (CallFunction|Set1Rotation 1 _returnvalue_2)
  (CallFunction|Set1Rotation 2 _returnvalue_2)
  (CallFunction|Set1Rotation 3 9e+01)
  (CallFunction|Set2Rotation 0 -9e+01)
  (CallFunction|Set2Rotation 1 _returnvalue_2)
  (CallFunction|Set2Rotation 2 _returnvalue_2)
  (CallFunction|Set2Rotation 3 9e+01)
  (CallFunction|Set3Rotation 0 -9e+01)
  (CallFunction|Set3Rotation 1 1.8e+02)
  (CallFunction|Set3Rotation 2 1.8e+02)
  (CallFunction|Set3Rotation 3 1.8e+02))

(event Custom|5%20Destroy%2030%25%20Door
  ;[1 1 1] 30% 문 파괴
  (Utilities|Array|Shuffle (Variables|Default|GetDoorWall))
  (for _index (range 0 (- (Utilities|Array|Length (Variables|Default|GetDoorWall)) 1))
    (Default|DestroyDoor (Utilities|Array|Get(acopy) (Variables|Default|GetDoorWall) _index)))
  (CallFunction|InitTP))

(event Custom|Destroy%20%20Unselected%20Room
  (for _array_element (Variables|RoomRef|Get2entrances)
    (if (== (Variables|/Game/Blueprint/Base/BP_BaseRoom.BP_BaseRoom_C|GetRoomIndex _array_element) -1)
      (Actor|DestroyActor _array_element)))
  (for _array_element_2 (Variables|RoomRef|Get3entrances)
    (if (== (Variables|/Game/Blueprint/Base/BP_BaseRoom.BP_BaseRoom_C|GetRoomIndex _array_element_2) -1)
      (Actor|DestroyActor _array_element_2)))
  (for _array_element_3 (Variables|RoomRef|Get4entrances)
    (if (== (Variables|/Game/Blueprint/Base/BP_BaseRoom.BP_BaseRoom_C|GetRoomIndex _array_element_3) -1)
      (Actor|DestroyActor _array_element_3)))
  (for _array_element_4 (Variables|RoomRef|Getkitchen)
    (if (== (Variables|/Game/Blueprint/Base/BP_BaseRoom.BP_BaseRoom_C|GetRoomIndex _array_element_4) -1)
      (Actor|DestroyActor _array_element_4))))

(event Custom|Add%202D%20Array%200
  (params (Target%20Item%20Array :type Array%20of%20BP%20Base%20Room%20Object%20References) (Item%20Index :type Integer))
  ;[1 1 1] 선택된 배열에 추가
  (Utilities|Array|Add (Variables|SelRoomRef|Get0) (Utilities|Array|Get(acopy) Target%20Item%20Array Item%20Index)))

(event Custom|Insert%20kitchen%20to%204
  (params (Index :type Integer) (Element :type BP%20Base%20Room%20Object%20Reference))
  (bind _2 (Variables|SelRoomRef|Get2))
  (bind _1 (Variables|SelRoomRef|Get1))
  ;[1 1 1] 부엌 교체 삽입 하드코딩
  (switch int Index
    (:0
      (Utilities|Array|SetArrayElem _1 1 Element)
      (Variables|Default|SetSelKitchen 4))
    (:1
      (Utilities|Array|SetArrayElem _1 2 Element)
      (Variables|Default|SetSelKitchen 5))
    (:2
      (Utilities|Array|SetArrayElem _2 1 Element)
      (Variables|Default|SetSelKitchen 8))
    (:3
      (Utilities|Array|SetArrayElem _2 2 Element)
      (Variables|Default|SetSelKitchen 9))))

(event Custom|Add%202D%20Array%201
  (params (Target%20Item%20Array :type Array%20of%20BP%20Base%20Room%20Object%20References) (Item%20Index :type Integer))
  ;[1 1 1] 선택된 배열에 추가
  (Utilities|Array|Add (Variables|SelRoomRef|Get1) (Utilities|Array|Get(acopy) Target%20Item%20Array Item%20Index)))

(event Custom|Insert%20Kitchen%20to%202
  (params (Index :type Integer) (Element :type BP%20Base%20Room%20Object%20Reference))
  (bind _0 (Variables|SelRoomRef|Get0))
  (bind _3 (Variables|SelRoomRef|Get3))
  ;[1 1 1] 부엌 교체 삽입 하드코딩
  (switch int Index
    (:0
      (Utilities|Array|SetArrayElem _0 0 Element)
      (Variables|Default|SetSelKitchen 0))
    (:1
      (Utilities|Array|SetArrayElem _0 3 Element)
      (Variables|Default|SetSelKitchen 3))
    (:2
      (Utilities|Array|SetArrayElem _3 0 Element)
      (Variables|Default|SetSelKitchen 12))
    (:3
      (Utilities|Array|SetArrayElem _3 3 Element)
      (Variables|Default|SetSelKitchen 15))))

(event Custom|Add%202D%20Array%202
  (params (Target%20Item%20Array :type Array%20of%20BP%20Base%20Room%20Object%20References) (Item%20Index :type Integer))
  ;[1 1 1] 선택된 배열에 추가
  (Utilities|Array|Add (Variables|SelRoomRef|Get2) (Utilities|Array|Get(acopy) Target%20Item%20Array Item%20Index)))

(event Custom|set%203%20Rotation
  (params (Index :type Integer) (Rotation%20Z :type Float%20%28single-precision%29))
  ;[1 1 1] 선택된 배열 회전 설정
  (Transformation|SetRelativeRotation (Variables|/Game/Blueprint/Base/BP_BaseRoom.BP_BaseRoom_C|GetDefaultSceneRoot (Utilities|Array|Get(acopy) (Variables|SelRoomRef|Get3) Index)) (Math|Rotator|MakeRotator 0.0 0.0 Rotation%20Z) false false))

(event Custom|Insert%20kitchen%20to%203
  (params (Index :type Integer) (Element :type BP%20Base%20Room%20Object%20Reference))
  (bind _0 (Variables|SelRoomRef|Get0))
  (bind _1 (Variables|SelRoomRef|Get1))
  (bind _2 (Variables|SelRoomRef|Get2))
  (bind _3 (Variables|SelRoomRef|Get3))
  ;[1 1 1] 부엌 교체 삽입 하드코딩
  (switch int Index
    (:0
      (Utilities|Array|SetArrayElem _0 1 Element)
      (Variables|Default|SetSelKitchen 1))
    (:1
      (Utilities|Array|SetArrayElem _0 2 Element)
      (Variables|Default|SetSelKitchen 2))
    (:2
      (Utilities|Array|SetArrayElem _1 0 Element)
      (Variables|Default|SetSelKitchen 4))
    (:3
      (Utilities|Array|SetArrayElem _1 3 Element)
      (Variables|Default|SetSelKitchen 7))
    (:4
      (Utilities|Array|SetArrayElem _2 0 Element)
      (Variables|Default|SetSelKitchen 8))
    (:5
      (Utilities|Array|SetArrayElem _2 3 Element)
      (Variables|Default|SetSelKitchen 11))
    (:6
      (Utilities|Array|SetArrayElem _3 1 Element)
      (Variables|Default|SetSelKitchen 13))
    (:7
      (Utilities|Array|SetArrayElem _3 2 Element)
      (Variables|Default|SetSelKitchen 14))))

(event Custom|Minus%20Room%20Score
  (params (TargetPoint :type BPT%20Location%20Point%20Object%20Reference))
  (bind _dic_lpscore (Variables|Default|GetDic_LPScore))
  (bind _value (Utilities|Map|Find _dic_lpscore TargetPoint))
  (if (> _value 1)
    (Utilities|Map|Add _dic_lpscore TargetPoint (- _value 1))
    (Development|PrintString (Utilities|String|Append (Utilities|String|Append (Utilities|String|Append "순찰갔더니 없네?" (Utilities|GetDisplayName TargetPoint)) "의 룸스코어 1점 하락 : ") (Utilities|String|ToString(Integer) (.Value (Utilities|Map|Find (Variables|Default|GetDic_LPScore) TargetPoint)))))))

(event Custom|Plus%20Room%20Score
  (params (TargetPoint :type BPT%20Location%20Point%20Object%20Reference))
  (bind _dic_lpscore (Variables|Default|GetDic_LPScore))
  (Utilities|Map|Add _dic_lpscore TargetPoint (+ (.Value (Utilities|Map|Find _dic_lpscore TargetPoint)) 5))
  (Development|PrintString (Utilities|String|Append (Utilities|String|Append (Utilities|String|Append "플레이어 발견으로 인한" (Utilities|GetDisplayName TargetPoint)) "의 룸스코어 상승 : ") (Utilities|String|ToString(Integer) (.Value (Utilities|Map|Find (Variables|Default|GetDic_LPScore) TargetPoint)))) true true "(R=1.000000,G=0.000000,B=0.872163,A=1.000000)"))

(fn ConstructionScript)

(fn GetSpawnPoint
  (if (> (Utilities|Array|Length (Variables|Default|GetSpawnTPConsumable)) 0)
    _
    (else
      (CallFunction|ReloadUniqueTP)))
  (LocalVariables|SetSelTP (Utilities|Array|Get(acopy) (Variables|Default|GetSpawnTPConsumable)))
  (Utilities|Array|RemoveIndex (Variables|Default|GetSpawnTPConsumable))
  (return (Transformation|GetActorLocation (LocalVariables|GetSelTP))))

(fn GetNearestPoint
  (params (TargetActor :type Actor%20Object%20Reference))
  (for (_array_element _array_index) (Variables|SelRoomRef|GetSelRoom)
    (if (< (Math|Vector|VectorLengthSquared (- (Transformation|GetActorLocation TargetActor) (Transformation|GetActorLocation _array_element))) (LocalVariables|GetMinLength))
      (LocalVariables|SetMinLength (Math|Vector|VectorLengthSquared (- (Transformation|GetActorLocation TargetActor) (Transformation|GetActorLocation _array_element))))
      (LocalVariables|SetSelRoomIndex _array_index)))
  (LocalVariables|SetMinLength 100000000376832.0)
  (bind _locationpoint (Default|GetLocationTP (Utilities|Array|Get(acopy) (Variables|SelRoomRef|GetSelRoom) (LocalVariables|GetSelRoomIndex))))
  (for (_array_element_2 _array_index_2) _locationpoint
    (if (< (Math|Vector|VectorLengthSquared (- (Transformation|GetActorLocation TargetActor) (Transformation|GetActorLocation _array_element_2))) (LocalVariables|GetMinLength))
      (LocalVariables|SetMinLength (Math|Vector|VectorLengthSquared (- (Transformation|GetActorLocation TargetActor) (Transformation|GetActorLocation _array_element_2))))
      (LocalVariables|SetSelPointIndex _array_index_2)))
  (return (Utilities|Array|Get(acopy) _locationpoint (LocalVariables|GetSelPointIndex))))