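; CH_Mom is the Mom character Blueprint, a set of events for driving her detection display, animation and movement.
; Detection feedback goes to a widget component's percent, a meter text, and head and body labels that toggle on or off.
; Montages are looked up by name in a map and printed when played, and the current one can be stopped.
; Movement events set the movement mode and switch between walk and run speed.
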(event Custom|set%20head
  (params (NewParam :type Boolean))
  (bind _head (Variables|Default|Gethead))
  (if NewParam
    (Rendering|Components|TextRender|SetText _head (Utilities|Text|MakeLiteralText "head"))
    (else
      (Rendering|Components|TextRender|SetText _head (Utilities|Text|MakeLiteralText "")))))

(event Custom|Play%20Anim
  (params (Montage%20Name :type Name))
  (Development|PrintString (Utilities|String|ToString(Name) Montage%20Name) true true "(R=0.064681,G=1.000000,B=0.000000,A=1.000000)")
  (Animation|PlayAnimMontage (.Value (Utilities|Map|Find (Variables|Default|GetDic_Montage) Montage%20Name)) 1.0 "None"))

(event Custom|Set%20Character%20Movemode
  (params (Can%20Move :type EMovementMode%20Enum :default "MOVE_None"))
  (Pawn|Components|CharacterMovement|SetMovementMode (Variables|Character|GetCharacterMovement) Can%20Move 0))

(event Custom|Set%20Mom%20Head%20Text2
  (params (Text :type String))
  (Rendering|Components|TextRender|SetText (Variables|Default|Getmeter) (Utilities|Text|ToText(String) Text)))

(event Custom|Stop%20Anim
  (bind _returnvalue (Animation|GetCurrentMontage :!class /Script/Engine.Character))
  (Utilities|IsValid _returnvalue
    (:Is%20Valid
      (Animation|StopAnimMontage _returnvalue))))

(event Custom|Set%20MoveSpeed
  (params (Run :type Boolean))
  (bind _charactermovement (Variables|Character|GetCharacterMovement))
  (if Run
    (Variables|/Script/Engine.CharacterMovementComponent|SetMaxWalkSpeed _charactermovement (Variables|Default|GetRunSpeed))
    (else
      (Variables|/Script/Engine.CharacterMovementComponent|SetMaxWalkSpeed _charactermovement (Variables|Default|GetWalkSpeed)))))

(event Custom|Set%20Eye%20Percent
  (params (Percent :type Float%20%28single-precision%29))
  (Default|SetDetectPercent (.AsWIdget%20Mom%20Detect (Utilities|Casting|CastToWIdget_MomDetect (UserInterface|GetUserWidgetObject (Variables|Default|GetDetect%20Widget)))) Percent))

(event Custom|set%20body
  (params (NewParam :type Boolean))
  (bind _body (Variables|Default|Getbody))
  (if NewParam
    (Rendering|Components|TextRender|SetText _body (Utilities|Text|MakeLiteralText "body"))
    (else
      (Rendering|Components|TextRender|SetText _body (Utilities|Text|MakeLiteralText "")))))

(fn ConstructionScript)