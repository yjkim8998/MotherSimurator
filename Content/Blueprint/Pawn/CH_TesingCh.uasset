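; CH_TesingCh is a test character that uses AI perception to track a VR player's head (BP_Head) and body (MotionControllerPawn) separately.
; Each perception update toggles the matching stored reference rather than reading the stimulus state.
; The DetectPlayer flag and text on W follow those references, with Head taking priority over Body.
; A slowed Tick draws a debug line to the detected head, falling back to the body.
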(event OnTargetPerceptionUpdated(AIPerception)
  (params (Actor :type Actor%20Object%20Reference) (Stimulus :type AI%20Stimulus%20Structure))
  (bind _returnvalue (Utilities|Text|MakeLiteralText "Body"))
  (bind _w (Variables|Default|Getw))
  (bind _w_2 (Variables|Default|Getw))
  (bind _asmotion_controller_pawn (Utilities|Casting|CastToMotionControllerPawn Actor)
    (:then
      (Utilities|IsValid (Variables|Default|GetPlayerBody)
        (:Is%20Valid
          (Variables|Default|SetPlayerBody 0)
          (Utilities|IsValid (Variables|Default|GetPlayerHead)
            (:Is%20Not%20Valid
              (Rendering|Components|TextRender|SetText _w (Utilities|Text|MakeLiteralText "None"))
              (Variables|Default|SetbDetectPlayer false))))
        (:Is%20Not%20Valid
          (Variables|Default|SetPlayerBody _asmotion_controller_pawn)
          (Utilities|IsValid (Variables|Default|GetPlayerHead)
            (:Is%20Not%20Valid
              (Rendering|Components|TextRender|SetText _w _returnvalue)
              (Variables|Default|SetbDetectPlayer true))))))
    (:CastFailed
      (bind _asbp_head (Utilities|Casting|CastToBP_Head Actor))
      (Utilities|IsValid (Variables|Default|GetPlayerHead)
        (:Is%20Valid
          (Variables|Default|SetPlayerHead 0)
          (Utilities|IsValid (Variables|Default|GetPlayerBody)
            (:Is%20Valid
              (Rendering|Components|TextRender|SetText _w_2 _returnvalue))
            (:Is%20Not%20Valid
              (Rendering|Components|TextRender|SetText _w_2 (Utilities|Text|MakeLiteralText "None"))
              (Variables|Default|SetbDetectPlayer false))))
        (:Is%20Not%20Valid
          (Variables|Default|SetPlayerHead _asbp_head)
          (Rendering|Components|TextRender|SetText _w_2 (Utilities|Text|MakeLiteralText "Head"))
          (Variables|Default|SetbDetectPlayer true))))))

(event EventTick
  (params (DeltaSeconds :type Float%20%28single-precision%29))
  (Utilities|IsValid (Variables|Default|GetPlayerHead)
    (:Is%20Valid
      (Rendering|Debug|DrawDebugLine (Transformation|GetActorLocation) (Transformation|GetActorLocation (Variables|Default|GetPlayerHead)) "(R=1.000000,G=0.043131,B=0.000000,A=1.000000)" 2.0 0.1))
    (:Is%20Not%20Valid
      (Utilities|IsValid (Variables|Default|GetPlayerBody)
        (:Is%20Valid
          (Rendering|Debug|DrawDebugLine (Transformation|GetActorLocation) (Transformation|GetActorLocation (Variables|Default|GetPlayerBody)) "(R=1.000000,G=0.043131,B=0.000000,A=1.000000)" 2.0 0.1))))))

(event EventBeginPlay
  (Actor|Tick|SetActorTickInterval 3.0))

(fn ConstructionScript)