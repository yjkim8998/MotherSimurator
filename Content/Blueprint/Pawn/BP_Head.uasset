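; BP_Head is a head actor that eats BP_BaseFood overlapping its Trigger volume and awards score for it.
; Trigger overlaps switch a one-second Tick on while food is inside and off when none remains, and each tick calls Eat on the overlapping food.
; Fully eaten food adds its score through GMBP_ScoreSystem, then returns to the ItemM pool or is destroyed.
; Capsule overlap events are empty, and camera fade calls are unconnected.
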(event OnComponentBeginOverlap(Capsule)
  (params (OverlappedComponent :type Primitive%20Component%20Object%20Reference) (OtherActor :type Actor%20Object%20Reference) (OtherComp :type Primitive%20Component%20Object%20Reference) (OtherBodyIndex :type Integer) (bFromSweep :type Boolean) (SweepResult :type Hit%20Result%20Structure%20%28by%20ref%29)))

(event OnComponentEndOverlap(Capsule)
  (params (OverlappedComponent :type Primitive%20Component%20Object%20Reference) (OtherActor :type Actor%20Object%20Reference) (OtherComp :type Primitive%20Component%20Object%20Reference) (OtherBodyIndex :type Integer)))

(event OnComponentBeginOverlap(Trigger)
  (params (OverlappedComponent :type Primitive%20Component%20Object%20Reference) (OtherActor :type Actor%20Object%20Reference) (OtherComp :type Primitive%20Component%20Object%20Reference) (OtherBodyIndex :type Integer) (bFromSweep :type Boolean) (SweepResult :type Hit%20Result%20Structure%20%28by%20ref%29))
  (Utilities|Casting|CastToBP_BaseFood OtherActor)
  (Actor|Tick|SetActorTickEnabled true))

(event OnComponentEndOverlap(Trigger)
  (params (OverlappedComponent :type Primitive%20Component%20Object%20Reference) (OtherActor :type Actor%20Object%20Reference) (OtherComp :type Primitive%20Component%20Object%20Reference) (OtherBodyIndex :type Integer))
  (Utilities|Casting|CastToBP_BaseFood OtherActor)
  (if (== (Utilities|Array|Length (Collision|GetOverlappingActors (Variables|Default|GetTrigger) "/Game/Blueprint/Base/BP_BaseFood.BP_BaseFood_C" :!class /Script/Engine.PrimitiveComponent)) 0)
    (Actor|Tick|SetActorTickEnabled false)))

(event EventTick
  (params (DeltaSeconds :type Float%20%28single-precision%29))
  (Development|PrintString "Hello")
  (for _array_element (Collision|GetOverlappingActors (Variables|Default|GetTrigger) "/Game/Blueprint/Base/BP_BaseFood.BP_BaseFood_C" :!class /Script/Engine.PrimitiveComponent)
    (bind _asbp_base_food (Utilities|Casting|CastToBP_BaseFood _array_element))
    (bind (_eat_all _food_ref) (Default|Eat _asbp_base_food))
    (if _eat_all
      (Default|PlusScore (.AsGMBP%20Score%20System (Utilities|Casting|CastToGMBP_ScoreSystem (Game|GetGameMode))) (Variables|/Game/Blueprint/Base/BP_BaseFood.BP_BaseFood_C|GetFoodScore _food_ref))
      (Utilities|IsValid (Variables|ManagerRef|GetItem%20M)
        (:Is%20Valid
          (Default|ReturnActortoPool (Variables|ManagerRef|GetItem%20M) _food_ref))
        (:Is%20Not%20Valid
          (Actor|DestroyActor _food_ref))))))

(event EventBeginPlay
  (Actor|Tick|SetActorTickInterval 1.0)
  (Actor|Tick|SetActorTickEnabled false))

(fn ConstructionScript)