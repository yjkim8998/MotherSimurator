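; BP_FryingPan is a cooking tool that can be picked up, dropped and used to cook food.
; Pickup attaches it with physics off; Drop re-enables physics and, given a valid Gasrange, snaps the mesh to the nearer burner target.
; Fire cooks food in the trigger whose cook types match the pan, emitting noise and sound.
; IsCookingWithFood tracks food presence while the range is on, refreshed on Fire and food leaving.
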(event OnComponentEndOverlap(Trigger)
  (params (OverlappedComponent :type Primitive%20Component%20Object%20Reference) (OtherActor :type Actor%20Object%20Reference) (OtherComp :type Primitive%20Component%20Object%20Reference) (OtherBodyIndex :type Integer))
  (Utilities|Casting|CastToBP_BaseCookFood OtherActor)
  (CallFunction|CheckCookwithFood))

(event Custom|Check%20Cook%20With%20Food
  (Utilities|IsValid (Variables|Default|GetGasrange)
    (:Is%20Valid
      (if (Variables|/Game/Blueprint/Furniture/Kitchen/BP_Induction.BP_Induction_C|GetTurnOnOff (Variables|Default|GetGasrange))
        (Variables|Default|SetIsCookingWithFood (> (Utilities|Array|Length (Collision|GetOverlappingActors (Variables|Default|GetTrigger) "/Game/Blueprint/Base/BP_BaseCookFOod.BP_BaseCookFood_C" :!class /Script/Engine.PrimitiveComponent)) 0))
        (else
          (Variables|Default|SetIsCookingWithFood false))))
    (:Is%20Not%20Valid
      (Variables|Default|SetIsCookingWithFood false))))

(event Custom|Fire
  (bind _trigger (Variables|Default|GetTrigger))
  (bind _overlappingactors (Collision|GetOverlappingActors _trigger "/Game/Blueprint/Base/BP_BaseCookFOod.BP_BaseCookFood_C" :!class /Script/Engine.PrimitiveComponent))
  (CallFunction|CheckCookwithFood)
  (if (> (Utilities|Array|Length _overlappingactors) 0)
    (Class|Actor|MakeNoise 1.0 (Game|Player|GetPlayerPawn 0) (Transformation|GetActorLocation) 0.0 "None")
    (for _array_element _overlappingactors
      (bind _asbp_base_cook_food (Utilities|Casting|CastToBP_BaseCookFood _array_element))
      (for _array_element_2 (Variables|/Game/Blueprint/Base/BP_BaseCookFOod.BP_BaseCookFood_C|GetCookType_food _asbp_base_cook_food)
        (if (== _array_element_2 (Variables|Default|GetCookType_tool))
          (Default|Cooking _asbp_base_cook_food)
          (Default|PlaySoundOnce (Variables|Default|GetCookingSoundController) "CookingSound")
          (Default|NoiseEvent (Variables|Default|GetCookingSoundController)))))))

(event EventBeginPlay
  (Variables|Default|SetCookType_tool "NewEnumerator0"))

(event EventPickup
  (params (AttachTo :type Scene%20Component%20Object%20Reference))
  (Physics|SetSimulatePhysics (Variables|Default|GetStaticMesh) false)
  (Transformation|AttachComponentToComponent (VehicleSound|GetRootComponent) AttachTo "None" "KeepWorld" "KeepWorld" "KeepWorld" false))

(event EventDrop
  (bind _gasrange (Variables|Default|GetGasrange))
  (bind _staticmesh (Variables|Default|GetStaticMesh))
  (bind _target1 (Variables|/Game/Blueprint/Furniture/Kitchen/BP_Induction.BP_Induction_C|GetTarget1 _gasrange))
  (bind _induction (Variables|/Game/Blueprint/Furniture/Kitchen/BP_Induction.BP_Induction_C|GetInduction _gasrange))
  (bind _target2 (Variables|/Game/Blueprint/Furniture/Kitchen/BP_Induction.BP_Induction_C|GetTarget2 _gasrange))
  (bind _returnvalue (Transformation|GetWorldLocation _target2))
  (bind _returnvalue_2 (Transformation|GetWorldLocation _target1))
  (bind _returnvalue_3 (Transformation|GetWorldRotation _induction))
  (bind (_roll _pitch _yaw) (Math|Rotator|BreakRotator _returnvalue_3))
  (bind _returnvalue_4 (- _yaw 9e+01))
  (bind _returnvalue_5 (Math|Rotator|MakeRotator _roll _pitch _returnvalue_4))
  (Physics|SetSimulatePhysics (Variables|Default|GetStaticMesh) true)
  (Transformation|DetachFromActor "KeepWorld" "KeepWorld" "KeepWorld")
  (Utilities|IsValid (Variables|Default|GetGasrange)
    (:Is%20Valid
      (if (< (Class|KismetMathLibrary|VectorDistanceSquared _returnvalue_2 (Transformation|GetWorldLocation _staticmesh)) (Class|KismetMathLibrary|VectorDistanceSquared _returnvalue (Transformation|GetWorldLocation _staticmesh)))
        (Transformation|SetRelativeLocationAndRotation (Variables|Default|GetStaticMesh) _returnvalue_2 _returnvalue_5 false false)
        (else
          (Transformation|SetRelativeLocationAndRotation (Variables|Default|GetStaticMesh) _returnvalue _returnvalue_5 false false))))))

(fn ConstructionScript)