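; BP_SinkTap is a kitchen sink tap whose valve is turned through a HandPoint component to switch a water particle effect on and off.
; Start and Stop toggle Tick and a gate, and Stop also realigns HandPoint.
; While active, Tick compares HandPoint yaw to the initial valve yaw and interpolates the valve toward it within angle limits.
; Passing a small threshold sets IsValveOn and starts the water trails once via DoOnce.
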(event EventBeginPlay
  (Effects|Particles|Trails|EndTrails (Variables|Default|GetWaterParticle))
  (Variables|Default|SetIsValveOn false)
  (Variables|Default|SetValveRotate (Math|Rotator|MakeRotator 0.0 0.0 (.Yaw (Math|Rotator|BreakRotator (Variables|/Script/Engine.SceneComponent|GetRelativeRotation (Variables|Default|GetSM_kitchen_sink_tap_valve)))))))

(event EventTick
  (params (DeltaSeconds :type Float%20%28single-precision%29))
  (bind _sm_kitchen_sink_tap_valve (Variables|Default|GetSM_kitchen_sink_tap_valve))
  (bind _sm_kitchen_sink_tap_valve_2 (Variables|Default|GetSM_kitchen_sink_tap_valve))
  (Utilities|FlowControl|Gate true
    (:Exit
      (Variables|Default|SetNewHandPointRotate (Math|Rotator|MakeRotator 0.0 0.0 (.Yaw (Math|Rotator|BreakRotator (Variables|/Script/Engine.SceneComponent|GetRelativeRotation (Variables|Default|GetHandPoint))))))
      (Variables|Default|SetCurrentAngle (- (.yaw (Variables|Default|GetNewHandPointRotate)) (.yaw (Variables|Default|GetValveRotate))))
      (if (> (Variables|Default|GetCurrentAngle) 2.0)
        (Variables|Default|SetIsValveOn true)
        (if (and (< (Variables|Default|GetCurrentAngle) (Variables|Default|GetMaxAngle)) (> (Variables|Default|GetCurrentAngle) (Variables|Default|GetMinAngle)))
          (Transformation|SetRelativeRotation _sm_kitchen_sink_tap_valve (Class|KismetMathLibrary|RInterptoConstant (Math|Rotator|MakeRotator 0.0 0.0 (.yaw (Variables|/Script/Engine.SceneComponent|GetRelativeRotation _sm_kitchen_sink_tap_valve))) (Variables|Default|GetNewHandPointRotate) (Utilities|Time|GetWorldDeltaSeconds) 0.0) false false)
          (Utilities|FlowControl|DoOnce false :!label _label
            (:Completed
              (Effects|Particles|Trails|BeginTrails (Variables|Default|GetWaterParticle) "None" "None" "ETrailWidthMode_FromCentre" 0.0))))
        (else
          (Variables|Default|SetIsValveOn false)
          (Effects|Particles|Trails|EndTrails (Variables|Default|GetWaterParticle))
          (if (and (< (Variables|Default|GetCurrentAngle) (Variables|Default|GetMaxAngle)) (> (Variables|Default|GetCurrentAngle) (Variables|Default|GetMinAngle)))
            (Transformation|SetRelativeRotation _sm_kitchen_sink_tap_valve_2 (Class|KismetMathLibrary|RInterptoConstant (Math|Rotator|MakeRotator 0.0 0.0 (.yaw (Variables|/Script/Engine.SceneComponent|GetRelativeRotation _sm_kitchen_sink_tap_valve_2))) (Variables|Default|GetNewHandPointRotate) (Utilities|Time|GetWorldDeltaSeconds) 0.0) false false)
            (goto _label Reset)))))))

(event EventStart
  (bind _sm_kitchen_sink_tap_valve (Variables|Default|GetSM_kitchen_sink_tap_valve))
  (bind _sm_kitchen_sink_tap_valve_2 (Variables|Default|GetSM_kitchen_sink_tap_valve))
  (Actor|Tick|SetActorTickEnabled true)
  (Utilities|FlowControl|Gate true) ; enters at Open
)

(event EventStop
  (bind _sm_kitchen_sink_tap_valve (Variables|Default|GetSM_kitchen_sink_tap_valve))
  (bind _sm_kitchen_sink_tap_valve_2 (Variables|Default|GetSM_kitchen_sink_tap_valve))
  (Actor|Tick|SetActorTickEnabled false)
  (Transformation|SetRelativeRotation (Variables|Default|GetHandPoint) (Variables|Default|GetNewHandPointRotate) false false)
  (Utilities|FlowControl|Gate true) ; enters at Close
)

(fn ConstructionScript)