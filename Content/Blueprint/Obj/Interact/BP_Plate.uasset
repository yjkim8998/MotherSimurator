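; BP_Plate is an interactable plate actor that can be picked up, dropped and broken on impact.
; Pickup turns off physics on the plate and attaches the actor to the given component, while Drop restores physics and detaches it.
; On Hit, when the hit component's speed times mass passes a threshold, it spawns BP_DestructiblePlate at the hit location and destroys itself.
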(event EventPickup
  (params (AttachTo :type Scene%20Component%20Object%20Reference))
  (Physics|SetSimulatePhysics (Variables|Default|GetPlate) false)
  (Transformation|AttachComponentToComponent (VehicleSound|GetRootComponent) AttachTo "None" "KeepWorld" "KeepWorld" "KeepWorld" false))

(event EventDrop
  (Physics|SetSimulatePhysics (Variables|Default|GetPlate) true)
  (Transformation|DetachFromActor "KeepWorld" "KeepWorld" "KeepWorld"))

(event Collision|EventHit
  (params (MyComp :type Primitive%20Component%20Object%20Reference) (Other :type Actor%20Object%20Reference) (OtherComp :type Primitive%20Component%20Object%20Reference) (bSelfMoved :type Boolean) (HitLocation :type Vector :default "0, 0, 0") (HitNormal :type Vector :default "0, 0, 0") (NormalImpulse :type Vector :default "0, 0, 0") (Hit :type Hit%20Result%20Structure%20%28by%20ref%29))
  (if (> (* (Math|Vector|VectorLength (Transformation|GetComponentVelocity MyComp)) (Physics|GetMass MyComp)) 5e+01)
    (Game|SpawnActorfromClass "/Game/Blueprint/Obj/Interact/BP_DestructiblePlate.BP_DestructiblePlate_C" (Math|Conversions|ToTransform(Vector) HitLocation) "Undefined" 0 0)
    (Actor|DestroyActor)))

(fn ConstructionScript)