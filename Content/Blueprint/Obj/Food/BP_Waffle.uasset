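; BP_Waffle is a food object whose score can be boosted by combining it with jam.
; On BeginPlay it rolls a random small FoodScore, copies it to FoodVolume, and sets its eat value and sound type.
; When an uncombined waffle's trigger overlaps a BP_Jam, it swaps the mesh material, triples FoodScore, marks itself combined and destroys the jam.
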(event OnComponentBeginOverlap(Trigger)
  (params (OverlappedComponent :type Primitive%20Component%20Object%20Reference) (OtherActor :type Actor%20Object%20Reference) (OtherComp :type Primitive%20Component%20Object%20Reference) (OtherBodyIndex :type Integer) (bFromSweep :type Boolean) (SweepResult :type Hit%20Result%20Structure%20%28by%20ref%29))
  (if (not (Variables|Default|GetIsCombined))
    (Utilities|Casting|CastToBP_Jam OtherActor)
    (Rendering|Material|SetMaterial (Variables|Default|GetStaticMesh) 0 "/Game/LMS/Materials/Water_Material.Water_Material")
    (Variables|Default|SetFoodScore (* (Variables|Default|GetFoodScore) 3.0))
    (Variables|Default|SetIsCombined true)
    (Actor|DestroyActor OtherActor)))

(event EventBeginPlay
  (bind _output_get (Variables|Default|SetFoodScore (Math|Conversions|ToFloat(Integer) (+ (Math|Random|RandomInteger 3) 1))))
  (Variables|Default|SetFoodVolume _output_get)
  (Variables|Default|SetEatValue 1.0)
  (Variables|Default|SetFoodSoundType "NewEnumerator2"))

(fn ConstructionScript)