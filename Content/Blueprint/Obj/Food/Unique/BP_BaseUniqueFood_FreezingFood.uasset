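; Base Blueprint for unique frozen food objects that show an icy coating over the food's mesh.
; On BeginPlay, after the parent logic, the FreezingFood mesh component copies the food's static mesh.
; It scales slightly larger than the base mesh and applies the IceFood material, forming an overlay shell rather than swapping the original material.
; The construction script only calls the parent.
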(event EventBeginPlay
  (|CallParentFunction)
  (Components|StaticMesh|SetStaticMesh (Variables|Default|GetFreezingFood) (Variables|/Script/Engine.StaticMeshComponent|GetStaticMesh (Variables|Default|GetStaticMesh)))
  (Transformation|SetRelativeScale3D (Variables|Default|GetFreezingFood) "1.010000,1.010000,1.010000")
  (Rendering|Material|SetMaterial (Variables|Default|GetFreezingFood) 0 "/Game/Z_JG/Material/IceFOod.IceFood"))

(fn ConstructionScript
  (|CallParentFunction))