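; BP_BaseUniqueFood is a base Blueprint for unique food objects tied to an event index.
; BeginPlay and Init both set a fixed food volume and copy it to the eat value, with Init also storing the event index.
; Destruction only prints a Korean debug message saying the food was eaten, as the event manager's finish call is unconnected.
; GetState always returns false.
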(event Custom|Init
  (params (Event%20Index :type Integer))
  (Variables|Default|SetEvent%20Index Event%20Index)
  (bind _output_get (Variables|Default|SetFoodVolume 3.0))
  (Variables|Default|SetEatValue _output_get))

(event EventBeginPlay
  (|CallParentFunction)
  (bind _output_get (Variables|Default|SetFoodVolume 3.0))
  (Variables|Default|SetEatValue _output_get))

(event EventDestroyed
  (Development|PrintString "음식을 먹었다"))

(fn ConstructionScript
  (|CallParentFunction))

(fn GetState
  (return false))