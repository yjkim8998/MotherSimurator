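; Unique egg food actor that turns into a fried egg when it hits something hard enough.
; On BeginPlay it sets its food score, volume, eat value and sound type, then shuffles three egg materials to give the mesh a random look.
; On a Hit, if its component velocity reaches a threshold, it spawns BP_Unique_Friedegg at the hit location and destroys itself.
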(event EventBeginPlay
  (bind _output_get (Variables|Default|SetFoodScore 1.0))
  (Variables|Default|SetFoodVolume _output_get)
  (Variables|Default|SetEatValue 1.0)
  (Variables|Default|SetFoodSoundType "NewEnumerator1")
  (bind _output_get_2 (Variables|Default|SetMaterial (Utilities|Array|MakeArray "/Game/Blueprint/Material/MI_egg_01.MI_egg_01" "/Game/Blueprint/Material/MI_egg_02.MI_egg_02" "/Game/Blueprint/Material/MI_egg_03.MI_egg_03")))
  (Utilities|Array|Shuffle _output_get_2)
  (Rendering|Material|SetMaterial (Variables|Default|GetStaticMesh) 0 (Utilities|Array|Get(acopy) _output_get_2)))

(event Collision|EventHit
  (params (MyComp :type Primitive%20Component%20Object%20Reference) (Other :type Actor%20Object%20Reference) (OtherComp :type Primitive%20Component%20Object%20Reference) (bSelfMoved :type Boolean) (HitLocation :type Vector :default "0, 0, 0") (HitNormal :type Vector :default "0, 0, 0") (NormalImpulse :type Vector :default "0, 0, 0") (Hit :type Hit%20Result%20Structure%20%28by%20ref%29))
  (if (>= (Math|Vector|VectorLength (Transformation|GetComponentVelocity MyComp)) 8e+01)
    (Game|SpawnActorfromClass "/Game/Blueprint/Obj/Food/Unique/BP_Unique_Friedegg.BP_Unique_Friedegg_C" (Math|Conversions|ToTransform(Vector) HitLocation) "Undefined" 0 0)
    (Actor|DestroyActor)))

(fn ConstructionScript)