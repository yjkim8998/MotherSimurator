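; Chicken food item that sets its own scoring, eating and cooking stats when play begins.
; BeginPlay rolls a small random FoodScore and derives FoodVolume and CookedScore from it as multiples.
; It also sets a fixed EatValue and perfectly-cooked level, then registers two cook types in CookTypeFood.
; The construction script is empty, and the Blueprint contains no other logic.
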(event EventBeginPlay
  (bind _output_get (Variables|Default|SetFoodScore (Math|Conversions|ToFloat(Integer) (+ (Math|Random|RandomInteger 5) 1))))
  (Variables|Default|SetFoodVolume (* _output_get 2.0))
  (Variables|Default|SetEatValue 1.0)
  (Variables|Default|SetPerfectelyCookedLevel 1e+01)
  (Variables|Default|SetCookedScore (* (Variables|Default|GetFoodScore) 3.0))
  (Utilities|Array|Add (Variables|Default|GetCookType_food) "NewEnumerator0")
  (Utilities|Array|Add (Variables|Default|GetCookType_food) "NewEnumerator2"))

(fn ConstructionScript)