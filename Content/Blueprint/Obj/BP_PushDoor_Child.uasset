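; BP_PushDoor_Child is a push door variant that swings open for AI crossing its child-actor smart nav link.
; On link reached, it snaps 90 degrees either way based on the destination's local X side.
; A 3-second timer resets rotation to zero; repeat triggers only restart it.
; If the mover is CH_Mom, its AI_Mom controller receives CheckNextRoom with the destination.
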(event Custom|AI%20Use%20link
  (params (MovingActor :type Actor%20Object%20Reference) (DestinationPoint :type Vector%20%28by%20ref%29))
  (CallFunction|CheckDir DestinationPoint)
  (bind _asch_mom (Utilities|Casting|CastToCH_Mom MovingActor))
  (bind _asai_mom (Utilities|Casting|CastToAI_Mom (Pawn|GetController _asch_mom)))
  (Default|CheckNextRoom _asai_mom DestinationPoint))

(event Custom|Check%20Dir
  (params (Destination :type Vector))
  (bind _returnvalue (Transformation|GetActorForwardVector))
  (bind _returnvalue_2 (Transformation|GetActorTransform))
  (bind _returnvalue_3 (Math|Transform|InverseTransformLocation _returnvalue_2 Destination))
  (if (Utilities|Time|IsValidTimerHandle (Variables|Default|GetRunningTimer))
    (Utilities|Time|ClearandInvalidateTimerbyHandle (Variables|Default|GetRunningTimer))
    (else
      (Development|PrintString "Hello" true true "(R=0.064681,G=0.000000,B=1.000000,A=1.000000)" 1e+01)
      (if (or (== (.x _returnvalue) 1.0) (== (.x _returnvalue) -1.0))
        (if (> (.x _returnvalue_3) 0.0)
          (Transformation|SetActorRelativeRotation "0,-90.000000, 0" :!label _label)
          (else
            (Transformation|SetActorRelativeRotation "0,90.000000, 0" :!label _label_2)))
        (elif (> (.x _returnvalue_3) 0.0)
          (goto _label)
          (else
            (goto _label_2))))))
  (bind _returnvalue_4 (Utilities|Time|SetTimerbyEvent (delegate Custom|Set%200%20Rotate) 3.0))
  (Variables|Default|SetRunningTimer _returnvalue_4))

(event Custom|Set%200%20Rotate
  (Transformation|SetActorRelativeRotation "0,0.000000, 0"))

(event EventBeginPlay
  (|CallParentFunction)
  (bind _asnav_link_proxy (Utilities|Casting|CastToNavLinkProxy (Variables|/Script/Engine.ChildActorComponent|GetChildActor (Variables|Default|GetNavLink))))
  (EventDispatchers|BindEventtoOnSmartLinkReached _asnav_link_proxy (delegate Custom|AI%20Use%20link)))

(event Collision|EventActorBeginOverlap
  (params (OtherActor :type Actor%20Object%20Reference))
  (|CallParentFunction OtherActor) ; 지금 이 노드는 비활성 상태입니다. \n핀을 끌어서 다른 노드를 연결하면 활성화됩니다.
)

(event EventTick
  (params (DeltaSeconds :type Float%20%28single-precision%29))
  (|CallParentFunction DeltaSeconds) ; 지금 이 노드는 비활성 상태입니다. \n핀을 끌어서 다른 노드를 연결하면 활성화됩니다.
)

(fn ConstructionScript
  (|CallParentFunction))