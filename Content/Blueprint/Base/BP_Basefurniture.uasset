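; Base furniture Blueprint that supplies its TP spawn entries to the room containing it.
; On BeginPlay it casts its parent actor to BP_BaseRoom and appends each BaseFunitureTP element to that room's BaseRoomTPSpawn list.
; GetTP exposes the same array.
; An identical registration loop sits disconnected in the construction script and never runs.
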(event EventBeginPlay
  (bind _asbp_base_room (Utilities|Casting|CastToBP_BaseRoom (Actor|GetParentActor)))
  (for _array_element (Variables|Default|GetBaseFunitureTP)
    (Utilities|Array|Add (Variables|/Game/Blueprint/Base/BP_BaseRoom.BP_BaseRoom_C|GetBaseRoomTP_Spawn _asbp_base_room) _array_element)))

(fn ConstructionScript)

(fn GetTP
  (return (Variables|Default|GetBaseFunitureTP)))