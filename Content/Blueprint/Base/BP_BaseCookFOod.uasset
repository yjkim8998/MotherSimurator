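; Base Blueprint for cookable food items that tracks a cook level and derives a food score from it.
; Each Cooking call raises CookedLevel by one and re-evaluates the score.
; A level within one step of the perfect value gives the cooked score, while going past it gives the overcooked score and blocks further cooking via a flag.
; ReturntoPool is overridden to hand the item back to ItemM's unique pool.
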(event Custom|Cooking
  (Variables|Default|SetCookedLevel (+ (Variables|Default|GetCookedLevel) 1.0))
  (CallFunction|SetFoodScore))

(event Custom|Set%20Food%20Score
  (if (Math|Float|InRange(Float) (Variables|Default|GetCookedLevel) (- (Variables|Default|GetPerfectelyCookedLevel) 1.0) (+ (Variables|Default|GetPerfectelyCookedLevel) 1.0))
    (Variables|Default|SetFoodScore (Variables|Default|GetCookedScore))
    (elif (> (Variables|Default|GetCookedLevel) (+ (Variables|Default|GetPerfectelyCookedLevel) 1.0)) ; Overcook
      (Variables|Default|SetFoodScore (Variables|Default|GetOverCookedScore))
      (Variables|Default|SetIsCannotCooking true))))

(event EventBeginPlay
  (|CallParentFunction))

(event EventReturntoPool
  (Default|ReturntoUniquePool (Variables|Default|GetItemM) self))

(fn ConstructionScript
  (|CallParentFunction))