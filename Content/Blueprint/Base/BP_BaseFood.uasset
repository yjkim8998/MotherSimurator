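; BP_BaseFood is a base food actor that a head collision actor eats over time.
; EatFoodEvent casts the input to BP_HeadCollision and, while it overlaps the food, loops with a one-second Delay, subtracting EatValue from FoodVolume and printing the result.
; The food destroys itself once FoodVolume equals exactly zero, and the loop stops when the overlap check fails.
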(event Custom|EatFoodEvent
  (params (InputHeadCollision :type Actor%20Object%20Reference))
  (bind _asbp_head_collision (Utilities|Casting|CastToBP_HeadCollision InputHeadCollision :!label _label))
  (if (Collision|IsOverlappingActor _asbp_head_collision :!class /Script/Engine.Actor)
    (if (== (Variables|Default|GetFoodVolume) 0.0)
      (Actor|DestroyActor)
      (else
        (Utilities|FlowControl|Delay 1.0)
        (bind _output_get (Variables|Default|SetFoodVolume (- (Variables|Default|GetFoodVolume) (Variables|Default|GetEatValue))))
        (Development|PrintString (Utilities|String|ToString(Float) _output_get))
        (goto _label)))))

(fn ConstructionScript)