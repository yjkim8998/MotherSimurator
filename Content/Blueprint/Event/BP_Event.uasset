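; BP_Event is a step-based gameplay event that completes when specific food items are eaten or overcooked.
; On begin, it asks EventM to spawn the current step's first condition target and binds to the manager's eat and overcook notifications.
; A food matching a current condition's type and target advances the step index.
; After the last step, it unbinds, resets and reports completion to EventM, with debug prints along the way.
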(event Custom|Clear%20Step%20Event
  (bind _result (Math|Integer|IncrementInt (Variables|Default|GetEventStepIndex))
    (:%20%20
      (if (== _result (Utilities|Array|Length (Variables|Default|GetEventSteps)))
        (CallFunction|EndEvent)))))

(event Custom|Check%20Eat%20Food
  (params (TargetFood :type BP%20Base%20Food%20Object%20Reference))
  ;[1 1 1] Check Condition
  (for _array_element (.eventcondition (Utilities|Array|Get(acopy) (Variables|Default|GetEventSteps) (Variables|Default|GetEventStepIndex)))
    (switch Utilities|FlowControl|Switch|SwitchonBPE_EventCompleteType (.eventtype _array_element)
      (:NewEnumerator0
        (if (== (.targetactor _array_element) TargetFood)
          (CallFunction|ClearStepEvent))))))

(event Custom|Check%20Over%20Cooked
  (params (TargetFood :type BP%20Base%20Food%20Object%20Reference))
  ;[1 1 1] Check Condition
  (Development|PrintString "Over Cook" true true "(R=1.000000,G=0.071315,B=0.000000,A=1.000000)" 5.0)
  (for _array_element (.eventcondition (Utilities|Array|Get(acopy) (Variables|Default|GetEventSteps) (Variables|Default|GetEventStepIndex)))
    (switch Utilities|FlowControl|Switch|SwitchonBPE_EventCompleteType (.eventtype _array_element)
      (:NewEnumerator1
        (if (== (.targetactor _array_element) TargetFood)
          (CallFunction|ClearStepEvent))))))

(event Custom|Bind%20Event
  (EventDispatchers|BindEventtoEatFood (Variables|ManagerRef|GetEventM) (EventDispatchers|CreateEvent :!event Custom|Check%20Eat%20Food))
  (EventDispatchers|BindEventtoOverCook (Variables|ManagerRef|GetEventM) (EventDispatchers|CreateEvent :!event Custom|Check%20Over%20Cooked)))

(event Custom|Begin%20Event
  (params (EventIndex :type Integer))
  (Variables|Default|SetEventIndex EventIndex)
  (Default|SpawnUniqueItemEvent (Variables|ManagerRef|GetEventM) (.targetactor (Utilities|Array|Get(acopy) (.eventcondition (Utilities|Array|Get(acopy) (Variables|Default|GetEventSteps) (Variables|Default|GetEventStepIndex))))))
  (CallFunction|BindEvent))

(event Custom|End%20Event
  (CallFunction|UnbindEvnet)
  (Variables|Default|SetEventStepIndex 0)
  (Default|EndEvent (Variables|ManagerRef|GetEventM) (Variables|Default|GetEventIndex))
  (Development|PrintString "이벤트 클리어 ㅁㅁㅁㅁㅁㅁㅁㅁㅁㅁㅁㅁㅁ" true true "(R=0.000000,G=0.024191,B=1.000000,A=1.000000)"))

(event Custom|Unbind%20Evnet
  (EventDispatchers|UnbindEventfromEatFood (Variables|ManagerRef|GetEventM) (EventDispatchers|CreateEvent :!event Custom|Check%20Eat%20Food))
  (EventDispatchers|UnbindEventfromOverCook (Variables|ManagerRef|GetEventM) (EventDispatchers|CreateEvent :!event Custom|Check%20Over%20Cooked)))

(fn ConstructionScript)