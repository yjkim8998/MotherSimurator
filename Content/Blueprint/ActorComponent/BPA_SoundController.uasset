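; Actor component that plays named sounds at its owner's location and reports noise events there.
; Sound names resolve through the DicSound map, either as fire-and-forget one-shots or as a single tracked PlayingSound.
; StopSound pauses that tracked sound, and PlaySound resumes it whatever name is passed, spawning a new one only when none is valid.
; NoiseEvent reports noise separately from playback, and the AIPerception RepNotify is empty.
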(event Custom|PlaySoundOnce
  (params (SoundName :type Name))
  (bind _dic_sound (Variables|Default|GetDic_Sound))
  (bind (_value _returnvalue) (Utilities|Map|Find _dic_sound SoundName))
  (if _returnvalue
    (Audio|PlaySoundatLocation _value (Transformation|GetActorLocation (Components|GetOwner)) "0, 0, 0" 1.0 1.0 0.0 0 0 0)))

(event Custom|PlaySound
  (params (SoundName :type Name))
  (bind _dic_sound (Variables|Default|GetDic_Sound))
  (bind (_value _returnvalue) (Utilities|Map|Find _dic_sound SoundName))
  (Utilities|IsValid (Variables|Default|GetPlayingSound)
    (:Is%20Valid
      (Class|AudioComponent|SetPaused (Variables|Default|GetPlayingSound) false))
    (:Is%20Not%20Valid
      (if _returnvalue
        (bind _returnvalue_2 (Audio|SpawnSoundatLocation _value (Transformation|GetActorLocation (Components|GetOwner)) "0, 0, 0" 1.0 1.0 0.0 0 0))
        (Variables|Default|SetPlayingSound _returnvalue_2)))))

(event Custom|StopSound
  (Utilities|IsValid (Variables|Default|GetPlayingSound)
    (:Is%20Valid
      (Class|AudioComponent|SetPaused (Variables|Default|GetPlayingSound) true))))

(event Custom|NoiseEvent
  (Class|AISenseHearing|ReportNoiseEvent (Transformation|GetActorLocation (Components|GetOwner)) 1.0 0 0.0 "None"))

(fn OnRepAIPerception)